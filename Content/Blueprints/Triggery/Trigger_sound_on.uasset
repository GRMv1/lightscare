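; Trigger actor that swaps between two referenced sound actors, SoundOn and SoundOff, as the FirstPersonCharacter enters and leaves it.
; On entry it fades out SoundOff, then activates and fades in SoundOn.
; On exit it fades SoundOff back in and calls Deactivate on SoundOn before its fade-out.
; Each fade-in starts playback at that sound actor's time since creation, so it resumes as if it had played continuously.
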(event `self.ReceiveActorBeginOverlap`
  (params (OtherActor :type "Actor Object Reference"))
  (bind _sound_on (`self.sound_on`))
  (bind _audiocomponent (`AmbientSound.AudioComponent` _sound_on))
  (cast `/Game/FirstPersonBP/Blueprints/FirstPersonCharacter` OtherActor)
  (`AudioComponent.FadeOut` (`AmbientSound.AudioComponent` (`self.sound_off`)) 1.0 0.0 "Linear")
  (`ActorComponent.Activate` _audiocomponent true)
  (`AudioComponent.FadeIn` _audiocomponent 0.3 1.0 (`self.GetGameTimeSinceCreation` _sound_on) "Linear"))

(event `self.ReceiveActorEndOverlap`
  (params (OtherActor :type "Actor Object Reference"))
  (bind _sound_off (`self.sound_off`))
  (bind _audiocomponent (`AmbientSound.AudioComponent` (`self.sound_on`)))
  (cast `/Game/FirstPersonBP/Blueprints/FirstPersonCharacter` OtherActor)
  (`AudioComponent.FadeIn` (`AmbientSound.AudioComponent` _sound_off) 0.3 1.0 (`self.GetGameTimeSinceCreation` _sound_off) "Linear")
  (`ActorComponent.Deactivate` _audiocomponent)
  (`AudioComponent.FadeOut` _audiocomponent 1.0 0.0 "Linear"))

(fn `UserConstructionScript`)