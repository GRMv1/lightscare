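; Petrol is a pickup actor that shows a "PressE" prompt widget while the FirstPersonCharacter is inside its Box trigger.
; Leaving the box removes the widget and disables the actor's input, though nothing here enables it.
; The custom event podnies (Polish for "pick up"), not called within this graph, destroys the actor and plays a sound at world origin.
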(event `podnies`
  (`self.K2_DestroyActor`)
  (`GameplayStatics.PlaySoundAtLocation` "/Game/Audio/Latarka/szuranie1_ciszej.szuranie1_ciszej" (0.0 0.0 0.0) (struct) 1.0 1.0 0.0 null null null))

(event `self.Box.OnComponentBeginOverlap`
  (params (OverlappedComponent :type "PrimitiveComponent Object Reference") (OtherActor :type "Actor Object Reference") (OtherComp :type "PrimitiveComponent Object Reference") (OtherBodyIndex :type Integer) (bFromSweep :type Boolean) (SweepResult :type "HitResult Structure (by ref)"))
  (cast `/Game/FirstPersonBP/Blueprints/FirstPersonCharacter` OtherActor)
  (bind _returnvalue (`|CreateWidget` "/Game/HUD/PressE.PressE_C" (`GameplayStatics.GetPlayerController` 0)))
  (`UserWidget.AddToViewport` _returnvalue 0))

(event `self.Box.OnComponentEndOverlap`
  (params (OverlappedComponent :type "PrimitiveComponent Object Reference") (OtherActor :type "Actor Object Reference") (OtherComp :type "PrimitiveComponent Object Reference") (OtherBodyIndex :type Integer))
  (cast `/Game/FirstPersonBP/Blueprints/FirstPersonCharacter` OtherActor)
  (`Widget.RemoveFromParent` (stale `self.Box.OnComponentBeginOverlap` _returnvalue))
  (`self.DisableInput` (`GameplayStatics.GetPlayerController` 0)))

(fn `UserConstructionScript`)