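; BP_Lampka is a lamp actor that can be switched on and off.
; On BeginPlay it creates a dynamic instance of M_Lamp on the second material slot of its static mesh and tints it pale yellow.
; TurnOn and TurnOff events switch that material's emission and the point light's visibility together, so the glow matches the light.
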(event `self.ReceiveBeginPlay`
  (bind _returnvalue (`PrimitiveComponent.CreateDynamicMaterialInstance` (`self.StaticMesh`) 1 "/Game/Materials/M_Lamp.M_Lamp" "None"))
  (bind _output_get (set `self.LampMaterial` _returnvalue))
  (`MaterialInstanceDynamic.SetVectorParameterValue` _output_get "Color" (struct :`R` 1.0 :`G` 1.0 :`B` 0.388235 :`A` 1.0)))

(event `TurnOn`
  (`MaterialInstanceDynamic.SetScalarParameterValue` (`self.LampMaterial`) "Emission" 10.0)
  (`SceneComponent.SetVisibility` (`self.PointLight`) true false))

(event `TurnOff`
  (`MaterialInstanceDynamic.SetScalarParameterValue` (`self.LampMaterial`) "Emission" 0.0)
  (`SceneComponent.SetVisibility` (`self.PointLight`) false false))

(fn `UserConstructionScript`)