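; Interactable switch actor (stun_switch) that slides its handle vertically when the player presses use nearby; no stun effect is wired here.
; Box overlap with FirstPersonCharacter shows a PressE widget and enables input, and leaving removes both.
; Timeline_0 drives the SwitchHandle's relative Z from the start on each press.
; Tick sets CanSwitch false while the timeline value is mid-travel, blocking presses in that range.
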(event `self.Box.OnComponentBeginOverlap`
  (params (OverlappedComponent :type "PrimitiveComponent Object Reference") (OtherActor :type "Actor Object Reference") (OtherComp :type "PrimitiveComponent Object Reference") (OtherBodyIndex :type Integer) (bFromSweep :type Boolean) (SweepResult :type "HitResult Structure (by ref)"))
  (bind _returnvalue (`GameplayStatics.GetPlayerController` 0))
  (cast `/Game/FirstPersonBP/Blueprints/FirstPersonCharacter` OtherActor)
  (bind _returnvalue_2 (`|CreateWidget` "/Game/HUD/PressE.PressE_C" _returnvalue))
  (`UserWidget.AddToViewport` _returnvalue_2 0)
  (`self.EnableInput` _returnvalue))

(event `self.Box.OnComponentEndOverlap`
  (params (OverlappedComponent :type "PrimitiveComponent Object Reference") (OtherActor :type "Actor Object Reference") (OtherComp :type "PrimitiveComponent Object Reference") (OtherBodyIndex :type Integer))
  (cast `/Game/FirstPersonBP/Blueprints/FirstPersonCharacter` OtherActor)
  (`Widget.RemoveFromParent` (stale `self.Box.OnComponentBeginOverlap` _returnvalue_2))
  (`self.DisableInput` (`GameplayStatics.GetPlayerController` 0)))

(event `InputAction|use`
  (params (Key :type "Key Structure"))
  (bind (_relativelocation_x _relativelocation_y) (`KismetMathLibrary.BreakVector` (`SceneComponent.RelativeLocation` (`self.switch_handle`))))
  (:`Pressed`
    (if (`self.can_switch`)
      (bind (_direction _switched) (`Timeline|Timeline_0` :!via `PlayFromStart`)
        (:`Update`
          (`SceneComponent.K2_SetRelativeLocation` (`self.switch_handle`) (`KismetMathLibrary.MakeVector` _relativelocation_x _relativelocation_y _switched) false false))))))

(event `self.ReceiveTick`
  (params (DeltaSeconds :type "Float (single-precision)"))
  (set `self.can_switch` (not (and (< (stale `InputAction|use` _switched) 125.0) (> (stale `InputAction|use` _switched) 16.0)))))

(fn `UserConstructionScript`)