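; Switch actor, apparently for a base generator, that toggles a set of linked lamps when its ToggleLamps event runs.
; It loops over the Lamps array, toggling visibility on a component reached by hard-coded child indices and flipping each lamp's IsLampOn flag.
; Each lamp triggers a sound at the switch's Cube: On_Cue when the flag becomes false, Off_Cue when it becomes true.
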(event `Toggle Lamps`
  (if true
    (for _array_element (`self.Lamps`)
      (`SceneComponent.ToggleVisibility` (`SceneComponent.GetChildComponent` (`SceneComponent.GetChildComponent` (`Actor.RootComponent` _array_element) 0) 0) false)
      (if (`/Game/Actors/Street_LampPrzyciagajacaPotwory.isLampOn` _array_element)
        (set `/Game/Actors/Street_LampPrzyciagajacaPotwory.isLampOn` false _array_element)
        (`GameplayStatics.PlaySoundAtLocation` "/Game/Audio/Latarka/On_Cue.On_Cue" (`SceneComponent.K2_GetComponentLocation` (`self.Cube`)) (struct) 1.0 1.0 0.0 null null null)
        (else
          (set `/Game/Actors/Street_LampPrzyciagajacaPotwory.isLampOn` true _array_element)
          (`GameplayStatics.PlaySoundAtLocation` "/Game/Audio/Latarka/Off_Cue.Off_Cue" (`SceneComponent.K2_GetComponentLocation` (`self.Cube`)) (struct) 1.0 1.0 0.0 null null null))))))

(fn `UserConstructionScript`)