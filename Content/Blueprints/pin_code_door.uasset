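; Sliding door actor that the player opens by entering a PIN code.
; A trigger box shows a PressE prompt and lets the use input open a keypad widget, which receives the code, freezes player movement and shows the cursor.
; The widget's dispatchers either re-arm the interaction or play a one-time timeline that slides the door along X and closes the gates on further overlap prompt handling.
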(event `self.Box.OnComponentBeginOverlap`
  (params (OverlappedComponent :type "PrimitiveComponent Object Reference") (OtherActor :type "Actor Object Reference") (OtherComp :type "PrimitiveComponent Object Reference") (OtherBodyIndex :type Integer) (bFromSweep :type Boolean) (SweepResult :type "HitResult Structure (by ref)"))
  (cast `/Game/FirstPersonBP/Blueprints/FirstPersonCharacter` OtherActor)
  (`/Engine/EditorBlueprintResources/StandardMacros.Gate` false :!label _label
    (:`Exit`
      (bind _returnvalue (`|CreateWidget` "/Game/HUD/PressE.PressE_C"))
      (`UserWidget.AddToViewport` _returnvalue 0)
      (set `self.near` true))))

(event `self.Box.OnComponentEndOverlap`
  (params (OverlappedComponent :type "PrimitiveComponent Object Reference") (OtherActor :type "Actor Object Reference") (OtherComp :type "PrimitiveComponent Object Reference") (OtherBodyIndex :type Integer))
  (cast `/Game/FirstPersonBP/Blueprints/FirstPersonCharacter` OtherActor)
  (`/Engine/EditorBlueprintResources/StandardMacros.Gate` false :!label _label_2
    (:`Exit`
      (bind _foundwidgets (`WidgetBlueprintLibrary.GetAllWidgetsOfClass` "/Game/HUD/PressE.PressE_C"))
      (`Widget.RemoveFromParent` (`|GetArrayItem` _foundwidgets))
      (set `self.near` false))))

(event `InputAction|use`
  (params (Key :type "Key Structure"))
  (bind _returnvalue (`GameplayStatics.GetPlayerController` 0))
  (:`Pressed`
    (if (`self.near`)
      (`/Engine/EditorBlueprintResources/StandardMacros.DoOnce` false :!label _label_3
        (:`Completed`
          (bind _returnvalue_2 (`|CreateWidget` "/Game/Blueprints/pin_code_widget.pin_code_widget_C"))
          (`UserWidget.AddToViewport` _returnvalue_2 0)
          (add `/Game/Blueprints/pin_code_widget.Reset` _returnvalue_2 (delegate `reset`))
          (add `/Game/Blueprints/pin_code_widget.OpenDoor` _returnvalue_2 (delegate `opendoor`))
          (set `/Game/Blueprints/pin_code_widget.PinCode` (`self.PinCode`) _returnvalue_2)
          (bind _outactors (`GameplayStatics.GetAllActorsOfClass` "/Game/FirstPersonBP/Blueprints/FirstPersonCharacter.FirstPersonCharacter_C"))
          (set `/Game/FirstPersonBP/Blueprints/FirstPersonCharacter.CanMove` false (`|GetArrayItem` _outactors))
          (set `PlayerController.bShowMouseCursor` true _returnvalue)
          (`Widget.SetUserFocus` _returnvalue_2 _returnvalue))))))

(event `reset`
  (goto _label_3 :!via `Reset`))

(event `opendoor`
  (bind _door (`self.door`))
  (bind (_relativelocation_x _relativelocation_y _relativelocation_z) (`KismetMathLibrary.BreakVector` (`SceneComponent.RelativeLocation` _door)))
  (`/Engine/EditorBlueprintResources/StandardMacros.DoOnce` false
    (:`Completed`
      (bind (_direction _move) (`Timeline|open`)
        (:`Update`
          (`SceneComponent.K2_SetRelativeLocation` _door (`KismetMathLibrary.MakeVector` _move _relativelocation_y _relativelocation_z) false false)
          (`|ExecutionSequence`
            (:`then_0`
              (goto _label :!via `Close`))
            (:`then_1`
              (goto _label_2 :!via `Close`))))))))

(fn `UserConstructionScript`)