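; Light-bearing actor that periodically lures nearby Mob_Ai enemies to itself.
; OnAttract starts a delayed cycle that toggles the PointLight and flip-flops mobs within range between Attract/NoMonsterNear and NoAttract/MonsterNear.
; The cycle re-arms through a Delay inside the mob loop, so it repeats only while a mob is in range.
; endAttract fires once, clearing the cycle flag after a delay and releasing nearby mobs if the lure is on.
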(event `OnAttract`
  (set `self.isAttract` true)
  (`KismetSystemLibrary.Delay` 8.0)
  (if (`self.isAttract`) :!label _label
    (`SceneComponent.ToggleVisibility` (`self.PointLight`) false)
    (`/Engine/EditorBlueprintResources/StandardMacros.FlipFlop`
      (:`A`
        (set `self.IsOn` true)
        (bind _outactors (`GameplayStatics.GetAllActorsOfClass` "/Game/ThirdPersonBP/AI/Mob_Ai.Mob_Ai_C"))
        (for _array_element _outactors
          (if (< (`KismetMathLibrary.Vector_Distance` (`self.K2_GetActorLocation` _array_element) (`self.K2_GetActorLocation`)) 2000.0)
            (`/Game/ThirdPersonBP/AI/Mob_Ai.noMonsterNear` _array_element)
            (`/Game/ThirdPersonBP/AI/Mob_Ai.attract` _array_element)
            (`KismetSystemLibrary.Delay` 16.0 :!label _label_2)
            (goto _label))))
      (:`B`
        (set `self.IsOn` false)
        (bind _outactors_2 (`GameplayStatics.GetAllActorsOfClass` "/Game/ThirdPersonBP/AI/Mob_Ai.Mob_Ai_C"))
        (for _array_element_2 _outactors_2
          (if (< (`KismetMathLibrary.Vector_Distance` (`self.K2_GetActorLocation` _array_element_2) (`self.K2_GetActorLocation`)) 2000.0)
            (`/Game/ThirdPersonBP/AI/Mob_Ai.noAttract` _array_element_2)
            (`/Game/ThirdPersonBP/AI/Mob_Ai.monsterNear` _array_element_2)
            (goto _label_2)))))))

(event `self.ReceiveBeginPlay`
  (`SceneComponent.ToggleVisibility` (`self.PointLight`) false))

(event `endAttract`
  (`/Engine/EditorBlueprintResources/StandardMacros.DoOnce` false
    (:`Completed`
      (`KismetSystemLibrary.Delay` 5.0)
      (set `self.isAttract` false)
      (if (`self.IsOn`)
        (`SceneComponent.ToggleVisibility` (`self.PointLight`) false)
        (set `self.IsOn` false)
        (bind _outactors (`GameplayStatics.GetAllActorsOfClass` "/Game/ThirdPersonBP/AI/Mob_Ai.Mob_Ai_C"))
        (for _array_element _outactors
          (if (< (`KismetMathLibrary.Vector_Distance` (`self.K2_GetActorLocation` _array_element) (`self.K2_GetActorLocation`)) 2000.0)
            (`/Game/ThirdPersonBP/AI/Mob_Ai.noAttract` _array_element)
            (`/Game/ThirdPersonBP/AI/Mob_Ai.monsterNear` _array_element)))))))

(fn `UserConstructionScript`)