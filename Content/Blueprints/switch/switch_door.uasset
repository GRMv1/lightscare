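; End-of-game door Blueprint that opens once the player has enabled the required number of switches.
; Box overlap shows a PressE widget, but enables input only if the character's SwitchWhichEnabled count equals AllSwitchPressed.
; The use action plays or reverses a timeline that yaws the door, with Tick deriving the closed state from the timeline value.
; When the timeline finishes, it shows the ENDGAME widget and loads MainMenu after a delay.
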(event `self.Box.OnComponentBeginOverlap`
  (params (OverlappedComponent :type "PrimitiveComponent Object Reference") (OtherActor :type "Actor Object Reference") (OtherComp :type "PrimitiveComponent Object Reference") (OtherBodyIndex :type Integer) (bFromSweep :type Boolean) (SweepResult :type "HitResult Structure (by ref)"))
  (bind _returnvalue (`GameplayStatics.GetPlayerController` 0))
  (bind _asfirst_person_character (cast `/Game/FirstPersonBP/Blueprints/FirstPersonCharacter` OtherActor))
  (bind _returnvalue_2 (`|CreateWidget` "/Game/HUD/PressE.PressE_C" _returnvalue))
  (`UserWidget.AddToViewport` _returnvalue_2 0)
  (if (== (`self.all_switch_pressed`) (`KismetArrayLibrary.Array_Length` (`/Game/FirstPersonBP/Blueprints/FirstPersonCharacter.switch_which_enabled` _asfirst_person_character)))
    (`self.EnableInput` _returnvalue)))

(event `self.Box.OnComponentEndOverlap`
  (params (OverlappedComponent :type "PrimitiveComponent Object Reference") (OtherActor :type "Actor Object Reference") (OtherComp :type "PrimitiveComponent Object Reference") (OtherBodyIndex :type Integer))
  (cast `/Game/FirstPersonBP/Blueprints/FirstPersonCharacter` OtherActor)
  (`Widget.RemoveFromParent` (stale `self.Box.OnComponentBeginOverlap` _returnvalue_2))
  (`self.DisableInput` (`GameplayStatics.GetPlayerController` 0)))

(event `InputAction|use`
  (params (Key :type "Key Structure"))
  (:`Pressed`
    (if (`self.closed_door`)
      (bind (_direction _door_open) (`Timeline|door rotation` :!label _label)
        (:`Update`
          (`SceneComponent.K2_SetRelativeRotation` (`self.door`) (`KismetMathLibrary.MakeRotator` 0.0 0.0 _door_open) false false))
        (:`Finished`
          (bind _returnvalue (`|CreateWidget` "/Game/HUD/ENDGAME.ENDGAME_C"))
          (`UserWidget.AddToViewport` _returnvalue 0)
          (`KismetSystemLibrary.Delay` 2.0)
          (`GameplayStatics.OpenLevel` "MainMenu")))
      (else
        (goto _label :!via `Reverse`)))))

(event `self.ReceiveTick`
  (params (DeltaSeconds :type "Float (single-precision)"))
  (set `self.closed_door` (< (stale `InputAction|use` _door_open) 1.0)))

(fn `UserConstructionScript`)