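; Manager actor that controls TriggerHint actors in bulk, selecting them by actor tag.
; SetTextToShowInTag updates the hint text and short-time flag on every match and optionally resets its counter.
; SetActorDisappeared toggles collision and tick on matches but always leaves them unhidden, despite its name.
; On BeginPlay it switches off collision and tick for hints tagged "police".
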(event `self.ReceiveBeginPlay`
  (`self.Set Actor Disappeared` "police" true))

(fn `Set Actor Disappeared`
  (params (tag :type Name) (`set disappeared` :type Boolean))
  (bind _returnvalue (not `set disappeared`))
  (bind _outactors (`GameplayStatics.GetAllActorsOfClassWithTag` "/Game/Blueprints/TriggerHint.TriggerHint_C" tag))
  (for _array_element _outactors
    (`self.SetActorHiddenInGame` _array_element false)
    (`self.SetActorEnableCollision` _array_element _returnvalue)
    (`self.SetActorTickEnabled` _array_element _returnvalue)))

(fn `SetTextToShowInTag`
  (params (tag :type Name) (newText :type String) (useShortTime :type Boolean) (resetCounter :type Boolean))
  (bind _outactors (`GameplayStatics.GetAllActorsOfClassWithTag` "/Game/Blueprints/TriggerHint.TriggerHint_C" tag))
  (for _array_element _outactors
    (set `/Game/Blueprints/TriggerHint.textToShow` newText _array_element)
    (set `/Game/Blueprints/TriggerHint.useShortTime` useShortTime _array_element)
    (if resetCounter
      (set `/Game/Blueprints/TriggerHint.counter` 0 _array_element))))

(fn `UserConstructionScript`)