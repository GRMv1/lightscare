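; Ambona light actor: a lamp that turns on when the player first enters its box and lures a monster.
; The one-shot overlap spawns a Mob at a fixed location, assigns its patrol path, passes flashlight and lamp state to Mob_Ai, and shows hints.
; Toggling the lamp updates the AI, hints and the player's UnderLamp fear flag.
; Checkpoint switches it off, rearms the trigger and removes any living monster, restarting Wire_trigger.
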(event `self.ReceiveBeginPlay`
  (`SceneComponent.SetVisibility` (`self.PointLight`) false false)
  (`SceneComponent.SetVisibility` (`self.PointLight1`) false false)
  (set `self.isOn` false))

(event `self.Box.OnComponentBeginOverlap`
  (params (OverlappedComponent :type "PrimitiveComponent Object Reference") (OtherActor :type "Actor Object Reference") (OtherComp :type "PrimitiveComponent Object Reference") (OtherBodyIndex :type Integer) (bFromSweep :type Boolean) (SweepResult :type "HitResult Structure (by ref)"))
  (bind _asfirst_person_character (cast `/Game/FirstPersonBP/Blueprints/FirstPersonCharacter` OtherActor))
  (`/Engine/EditorBlueprintResources/StandardMacros.DoOnce` false :!label _label
    (:`Completed`
      (`SceneComponent.SetVisibility` (`self.PointLight`) true false)
      (`SceneComponent.SetVisibility` (`self.PointLight1`) true false)
      (set `self.isOn` true)
      (`self.updateFear`)
      (bind _outactors (`GameplayStatics.GetAllActorsOfClass` "/Game/ThirdPersonBP/AI/PatrolPath.PatrolPath_C"))
      (for _array_element _outactors
        (if (`self.ActorHasTag` _array_element (`|GetArrayItem` (`Actor.Tags` _array_element)))
          (bind _value_ (`|LowEntry_LocalVariable` _array_element))
          (bind _returnvalue (`AIBlueprintHelperLibrary.SpawnAIFromClass` "/Game/ThirdPersonBP/AI/Mob.Mob_C" "/Game/ThirdPersonBP/AI/Mob_BehaviourTree.Mob_BehaviourTree" (-2991.393799 83208.351562 423.408691) (struct) false null))
          (bind _asmob (cast `/Game/ThirdPersonBP/AI/Mob` _returnvalue))
          (set `/Game/ThirdPersonBP/AI/Mob.PatrolPath` _value_ _asmob)
          (bind _asmob_ai (cast `/Game/ThirdPersonBP/AI/Mob_Ai` (`Pawn.GetController` _asmob)))
          (set `/Game/ThirdPersonBP/AI/Mob_Ai.MyPawn` _asmob _asmob_ai)
          (set `self.isMonsterAlive` true)
          (if (`/Game/FirstPersonBP/Blueprints/FirstPersonCharacter.is_light_on` _asfirst_person_character)
            (`/Game/ThirdPersonBP/AI/Mob_Ai.SetFlashlightOn` _asmob_ai)
            (else
              (`/Game/ThirdPersonBP/AI/Mob_Ai.SetFlashlightOff` _asmob_ai)))
          (`/Game/ThirdPersonBP/AI/Mob_Ai.SetIsAmbonaLightOnTrue` _asmob_ai)
          (bind _returnvalue_2 (`GameplayStatics.GetActorOfClass` "/Game/Blueprints/TriggerHintManager.TriggerHintManager_C"))
          (`/Game/Blueprints/TriggerHintManager.SetTextToShowInTag` _returnvalue_2 "ambona" "Hmm... Light seems to attract monster. Maybe i should try turn off the light." true true)
          (`KismetSystemLibrary.Delay` 1.0)
          (bind _foundwidgets (`WidgetBlueprintLibrary.GetAllWidgetsOfClass` "/Game/HUD/text_bot_screen.text_bot_screen_C"))
          (`/Game/HUD/text_bot_screen.ShowMessage` :`self` _foundwidgets :`text` "What is that creature? It has probably been lured by the light." :`time` 3.0))))))

(event `Reset Light Ambona`
  (goto _label :!via `Reset`))

(event `TurnOnOffAmbonaLight`
  (bind _returnvalue (not (`self.isOn`)))
  (`SceneComponent.SetVisibility` (`self.PointLight`) _returnvalue false)
  (`SceneComponent.SetVisibility` (`self.PointLight1`) _returnvalue false)
  (set `self.isOn` _returnvalue)
  (`self.updateFear`)
  (bind _asmob (cast `/Game/ThirdPersonBP/AI/Mob` (stale `self.Box.OnComponentBeginOverlap` _returnvalue)))
  (bind _asmob_ai (cast `/Game/ThirdPersonBP/AI/Mob_Ai` (`Pawn.GetController` _asmob)))
  (if (`self.isOn`)
    (`/Game/ThirdPersonBP/AI/Mob_Ai.SetIsAmbonaLightOnTrue` _asmob_ai)
    (bind _returnvalue_2 (`GameplayStatics.GetActorOfClass` "/Game/Blueprints/TriggerHintManager.TriggerHintManager_C"))
    (`/Game/Blueprints/TriggerHintManager.SetTextToShowInTag` _returnvalue_2 "ambona" "Hmm... light seems to attract monsters. Maybe i should try turn of the light." false false)
    (else
      (`/Game/ThirdPersonBP/AI/Mob_Ai.SetIsAmbonaLightFalse` _asmob_ai)
      (bind _returnvalue_3 (`GameplayStatics.GetActorOfClass` "/Game/Blueprints/TriggerHintManager.TriggerHintManager_C"))
      (`/Game/Blueprints/TriggerHintManager.SetTextToShowInTag` _returnvalue_3 "ambona" "Maybe I should use flashlight to distract the monster." false false))))

(event `checkpoint`
  (`SceneComponent.SetVisibility` (`self.PointLight`) false false)
  (`SceneComponent.SetVisibility` (`self.PointLight1`) false false)
  (set `self.isOn` false)
  (`self.updateFear`)
  (if (`self.isMonsterAlive`)
    (bind _asmob (cast `/Game/ThirdPersonBP/AI/Mob` (stale `self.Box.OnComponentBeginOverlap` _returnvalue)))
    (bind _asmob_ai (cast `/Game/ThirdPersonBP/AI/Mob_Ai` (`Pawn.GetController` _asmob)))
    (`self.K2_DestroyActor` _asmob_ai)
    (`self.K2_DestroyActor` (stale `self.Box.OnComponentBeginOverlap` _returnvalue))
    (`self.Reset Light Ambona`)
    (bind _returnvalue (`GameplayStatics.GetActorOfClass` "/Game/Actors/Wire_trigger.Wire_trigger_C"))
    (`/Game/Actors/Wire_trigger.RestartWireTrigger` _returnvalue)
    (else
      (`self.Reset Light Ambona`)
      (bind _returnvalue_2 (`GameplayStatics.GetActorOfClass` "/Game/Blueprints/TriggerHintManager.TriggerHintManager_C"))
      (`/Game/Blueprints/TriggerHintManager.Set Actor Disappeared` _returnvalue_2 "ambona" false))))

(event `updateFear`
  (bind _asfirst_person_character (cast `/Game/FirstPersonBP/Blueprints/FirstPersonCharacter` (`GameplayStatics.GetPlayerCharacter` 0)))
  (set `/Game/FirstPersonBP/Blueprints/FirstPersonCharacter.under_lamp` (`self.isOn`) _asfirst_person_character))

(fn `UserConstructionScript`)