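; Interactable rack that the player can push once, playing a sound and triggering a story hint about monsters outside.
; Box overlap toggles player input and interaction flags until the rack has been pushed.
; Pressing pick_up while hovered runs a one-shot Push timeline that pitches the Sphere component.
; When it finishes, the rack is marked pushed and inactive, the audio stops and the bottom-screen text widget shows the hint.
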(event `self.ReceiveBeginPlay`
  (`parent.ReceiveBeginPlay`)
  (set `self.Discovered` true))

(event `self.Box.OnComponentBeginOverlap`
  (params (OverlappedComponent :type "PrimitiveComponent Object Reference") (OtherActor :type "Actor Object Reference") (OtherComp :type "PrimitiveComponent Object Reference") (OtherBodyIndex :type Integer) (bFromSweep :type Boolean) (SweepResult :type "HitResult Structure (by ref)"))
  (bind _returnvalue (`GameplayStatics.GetPlayerController` 0))
  (if (`self.pushed`)
    (set `self.Active` false)
    (`self.DisableInput` _returnvalue :!label _label)
    (else
      (set `self.Active` true)
      (if (== OtherActor (cast `/Game/FirstPersonBP/Blueprints/FirstPersonCharacter` (`GameplayStatics.GetPlayerCharacter` 0) :!pure true))
        (set `self.Can_interact` true)
        (`self.EnableInput` _returnvalue)))))

(event `self.Box.OnComponentEndOverlap`
  (params (OverlappedComponent :type "PrimitiveComponent Object Reference") (OtherActor :type "Actor Object Reference") (OtherComp :type "PrimitiveComponent Object Reference") (OtherBodyIndex :type Integer))
  (if (== (cast `/Game/FirstPersonBP/Blueprints/FirstPersonCharacter` (`GameplayStatics.GetPlayerCharacter` 0) :!pure true) OtherActor)
    (set `self.Can_interact` false)
    (goto _label)))

(event `InputAction|pick_up`
  (params (Key :type "Key Structure"))
  (bind (_relativerotation_roll _relativerotation_pitch _relativerotation_yaw) (`KismetMathLibrary.BreakRotator` (`SceneComponent.RelativeRotation` (`self.Sphere`))))
  (:`Pressed`
    (if (`self.Hovered`)
      (`AudioComponent.Play` (`self.audio`) 0.0)
      (`/Engine/EditorBlueprintResources/StandardMacros.DoOnce` false
        (:`Completed`
          (bind (_direction _push) (`Timeline|push`)
            (:`Update`
              (`SceneComponent.K2_SetRelativeRotation` (`self.Sphere`) (`KismetMathLibrary.MakeRotator` _relativerotation_roll _push _relativerotation_yaw) false false))
            (:`Finished`
              (set `self.pushed` true)
              (bind _foundwidgets (`WidgetBlueprintLibrary.GetAllWidgetsOfClass` "/Game/HUD/text_bot_screen.text_bot_screen_C"))
              (`/Game/HUD/text_bot_screen.ShowMessage` :`self` _foundwidgets :`text` "I hear monsters outside, is there anything I can use to drive them away?" :`time` 3.0)
              (`AudioComponent.Stop` (`self.audio`))
              (set `self.Active` false))))))))

(fn `UserConstructionScript`
  (`parent.UserConstructionScript`))