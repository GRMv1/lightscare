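; Interactable high-voltage cable box that the player repairs by holding pick_up for two seconds while it is hovered and discovered.
; Tick rotates the box from key hold time and manages a hold-E prompt, while collision overlap toggles input.
; A Hold macro built from a retriggerable delay and gates completes the repair: sparks and sound stop, broken cable switches are fixed, light switches update, and a timeline turns the arrow.
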(event `self.ReceiveBeginPlay`
  (`parent.ReceiveBeginPlay`)
  (set `self.Discovered` false)
  (`AudioComponent.Play` (`self.high_voltage_Cue`) 0.0)
  (`ActorComponent.Activate` (`self.spiecie`) false))

(event `self.ReceiveTick`
  (params (DeltaSeconds :type "Float (single-precision)"))
  (set `self.hold_value` (`PlayerController.GetInputKeyTimeDown` (`GameplayStatics.GetPlayerController` 0) (stale `InputAction|pick_up` Key)))
  (`parent.ReceiveTick` DeltaSeconds)
  (if (`self.Hovered`)
    (if (`self.Discovered`)
      (if (`PrimitiveComponent.IsOverlappingComponent` (`Character.CapsuleComponent` (`GameplayStatics.GetPlayerCharacter` 0)) (`self.Collision`))
        (if (`self.was_used`)
          (if (`self.widgetAlive`) :!label _label
            (`Widget.RemoveFromParent` (stale `self.ReceiveTick` _returnvalue))
            (goto _label_2 :!via `Reset`))
          (else
            (`SceneComponent.K2_SetRelativeRotation` (`self.doZwiekszeniaEnergiiPudelko_DoObracania`) (`KismetMathLibrary.MakeRotator` (* (`self.hold_value`) -90.0) 0.0 90.0) false false)
            (`/Engine/EditorBlueprintResources/StandardMacros.DoOnce` false :!label _label_2
              (:`Completed`
                (bind _returnvalue (`|CreateWidget` "/Game/HUD/HoldE.HoldE_C"))
                (`UserWidget.AddToViewport` _returnvalue 0)
                (set `self.widgetAlive` true)))))
        (else
          (goto _label))))
    (else
      (goto _label))))

(event `InputAction|pick_up`
  (params (Key :type "Key Structure"))
  (bind _returnvalue (`GameplayStatics.GetPlayerController` 0))
  (bind _returnvalue_2 (`GameplayStatics.GetPlayerCharacter` 0))
  (bind _returnvalue_3 (`GameplayStatics.GetPlayerController` 0))
  (:`Pressed`
    (if (`self.Hovered`)
      (if (`self.Discovered`)
        (`self.DisableInput` _returnvalue_2 _returnvalue_3)
        (`self.Hold` 2.0 :!label _label_3
          (:`Held`
            (`SceneComponent.SetVisibility` (`self.spiecie`) false false)
            (`AudioComponent.Stop` (`self.high_voltage_Cue`))
            (bind _outactors (`GameplayStatics.GetAllActorsOfClass` "/Game/Blueprints/PickUp/broken_switch_kable.broken_switch_kable_C"))
            (for _array_element _outactors
              (set `/Game/Blueprints/PickUp/broken_switch_kable.is_broken` false _array_element))
            (set `self.was_used` true)
            (if (`self.widgetAlive`)
              (`Widget.RemoveFromParent` (stale `self.ReceiveTick` _returnvalue))
              (set `self.widgetAlive` false))
            (bind _outactors_2 (`GameplayStatics.GetAllActorsOfClass` "/Game/Blueprints/przelacznik/switch_light_broken.switch_light_broken_C"))
            (for _array_element_2 _outactors_2
              (`/Game/Blueprints/przelacznik/switch_light_broken.SwitchLightRedOrYellowKable` _array_element_2)
              (bind (_direction _newtrack_0) (`Timeline|strzalka`)
                (:`Update`
                  (`SceneComponent.K2_SetRelativeRotation` (`self.doZwiekszeniaEnergiiPudelko_strzałka`) (`KismetMathLibrary.MakeRotator` _newtrack_0 0.0 90.0) false false))
                (:`Finished`
                  (`self.EnableInput` (`GameplayStatics.GetPlayerCharacter` 0) _returnvalue)
                  (`self.DisableInput` _returnvalue)
                  (set `self.Active` false)))))))))
  (:`Released`
    (`self.EnableInput` _returnvalue_2 _returnvalue_3)
    (goto _label_3 :!via `released`)))

(event `self.Collision.OnComponentBeginOverlap`
  (params (OverlappedComponent :type "PrimitiveComponent Object Reference") (OtherActor :type "Actor Object Reference") (OtherComp :type "PrimitiveComponent Object Reference") (OtherBodyIndex :type Integer) (bFromSweep :type Boolean) (SweepResult :type "HitResult Structure (by ref)"))
  (bind _returnvalue (`GameplayStatics.GetPlayerController` 0))
  (if (== OtherActor (cast `/Game/FirstPersonBP/Blueprints/FirstPersonCharacter` (`GameplayStatics.GetPlayerCharacter` 0) :!pure true))
    (set `self.Can_interact` true)
    (if (`self.was_used`)
      (set `self.Active` false)
      (`self.DisableInput` _returnvalue :!label _label_4)
      (else
        (`self.EnableInput` _returnvalue)))))

(event `self.Collision.OnComponentEndOverlap`
  (params (OverlappedComponent :type "PrimitiveComponent Object Reference") (OtherActor :type "Actor Object Reference") (OtherComp :type "PrimitiveComponent Object Reference") (OtherBodyIndex :type Integer))
  (if (== (cast `/Game/FirstPersonBP/Blueprints/FirstPersonCharacter` (`GameplayStatics.GetPlayerCharacter` 0) :!pure true) OtherActor)
    (set `self.Can_interact` false)
    (if (`self.was_used`)
      (goto _label_4)
      (else
        (goto _label_4)))))

(fn `UserConstructionScript`
  (`parent.UserConstructionScript`))