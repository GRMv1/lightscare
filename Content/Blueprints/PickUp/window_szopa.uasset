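; Interactive shed window that the player swings open and closed with the pick_up input.
; A box overlap toggles CanInteract and enables or disables input for the player character.
; When Hovered and Discovered (set true on BeginPlay), each press alternates playing and reversing the Open timeline, whose two tracks yaw the two panes.
; CanInteract is not checked in this graph, and Hovered is not set here.
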(event `self.ReceiveBeginPlay`
  (`parent.ReceiveBeginPlay`)
  (set `self.Discovered` true))

(event `self.Box.OnComponentBeginOverlap`
  (params (OverlappedComponent :type "PrimitiveComponent Object Reference") (OtherActor :type "Actor Object Reference") (OtherComp :type "PrimitiveComponent Object Reference") (OtherBodyIndex :type Integer) (bFromSweep :type Boolean) (SweepResult :type "HitResult Structure (by ref)"))
  (if (== OtherActor (cast `/Game/FirstPersonBP/Blueprints/FirstPersonCharacter` (`GameplayStatics.GetPlayerCharacter` 0) :!pure true))
    (set `self.Can_interact` true)
    (`self.EnableInput` (`GameplayStatics.GetPlayerController` 0))))

(event `self.Box.OnComponentEndOverlap`
  (params (OverlappedComponent :type "PrimitiveComponent Object Reference") (OtherActor :type "Actor Object Reference") (OtherComp :type "PrimitiveComponent Object Reference") (OtherBodyIndex :type Integer))
  (if (== (cast `/Game/FirstPersonBP/Blueprints/FirstPersonCharacter` (`GameplayStatics.GetPlayerCharacter` 0) :!pure true) OtherActor)
    (set `self.Can_interact` false)
    (`self.DisableInput` (`GameplayStatics.GetPlayerController` 0))))

(event `InputAction|pick_up`
  (params (Key :type "Key Structure"))
  (:`Pressed`
    (if (`self.Hovered`)
      (if (`self.Discovered`)
        (`/Engine/EditorBlueprintResources/StandardMacros.FlipFlop`
          (:`A`
            (bind (_direction _newtrack_0 _newtrack_1) (`Timeline|open` :!label _label)
              (:`Update`
                (`SceneComponent.K2_SetRelativeRotation` (`self.window_p1`) (`KismetMathLibrary.MakeRotator` 0.0 0.0 _newtrack_0) false false)
                (`SceneComponent.K2_SetRelativeRotation` (`self.window_p2`) (`KismetMathLibrary.MakeRotator` 0.0 0.0 _newtrack_1) false false))))
          (:`B`
            (goto _label :!via `Reverse`)))))))

(fn `UserConstructionScript`
  (`parent.UserConstructionScript`))