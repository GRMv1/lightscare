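; Breakable switch actor that, unless flagged IsBroken, flips once when the pick_up input is pressed.
; Flipping appends a false entry to the player's SwitchWhichEnabled array, sets SwitchEnabled and plays a sound at the Sphere's relative location.
; It then calls SwitchLight on every Switch_light actor and plays a timeline that slides the handle along Z.
; The graph itself has no overlap or range check.
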(event `InputAction|pick_up`
  (params (Key :type "Key Structure"))
  (bind (_relativelocation_x _relativelocation_y) (`KismetMathLibrary.BreakVector` (`SceneComponent.RelativeLocation` (`self.switch_handle`))))
  (:`Pressed`
    (if (not (`self.is_broken`))
      (`/Engine/EditorBlueprintResources/StandardMacros.DoOnce` false
        (:`Completed`
          (bind _asfirst_person_character (cast `/Game/FirstPersonBP/Blueprints/FirstPersonCharacter` (`GameplayStatics.GetPlayerCharacter` 0)))
          (bind _switch_which_enabled (`/Game/FirstPersonBP/Blueprints/FirstPersonCharacter.switch_which_enabled` _asfirst_person_character))
          (`KismetArrayLibrary.Array_Add` _switch_which_enabled)
          (set `self.switch_enabled` true)
          (`GameplayStatics.PlaySoundAtLocation` "/Game/Audio/przelacznik/switch.switch" (`SceneComponent.RelativeLocation` (`self.Sphere`)) (struct) 1.0 1.0 0.0 null null null)
          (bind _outactors (`GameplayStatics.GetAllActorsOfClass` "/Game/Blueprints/przelacznik/switch_light.switch_light_C"))
          (for _array_element _outactors
            (`/Game/Blueprints/przelacznik/switch_light.SwitchLight` _array_element)
            (for _ _switch_which_enabled
              (bind (_direction _switched) (`Timeline|Timeline_1`)
                (:`Update`
                  (`SceneComponent.K2_SetRelativeLocation` (`self.switch_handle`) (`KismetMathLibrary.MakeVector` _relativelocation_x _relativelocation_y _switched) false false))))))))))

(fn `UserConstructionScript`
  (`parent.UserConstructionScript`))