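; Flashlight pickup actor that gives the first-person character a flashlight.
; Overlap with its Collision component toggles input and a CanInteract flag for the player.
; Pressing pick_up while interactable, hovered and discovered sets HasFlashlight and IsDestroyedPickupItem on the character once, then destroys the actor.
; Hovered, Discovered and PlayerRef are read here but not set in this graph.
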(event `InputAction|pick_up`
  (params (Key :type "Key Structure"))
  (:`Pressed`
    (if (and (`self.Can_interact`) (`self.Hovered`) (`self.Discovered`))
      (`/Engine/EditorBlueprintResources/StandardMacros.DoOnce` false
        (:`Completed`
          (bind _asfirst_person_character (cast `/Game/FirstPersonBP/Blueprints/FirstPersonCharacter` (`GameplayStatics.GetPlayerCharacter` 0)))
          (set `/Game/FirstPersonBP/Blueprints/FirstPersonCharacter.has_flashlight` true _asfirst_person_character)
          (set `/Game/FirstPersonBP/Blueprints/FirstPersonCharacter.is_destroyed_pickup_item` true _asfirst_person_character)
          (`self.K2_DestroyActor`))))))

(event `self.Collision.OnComponentBeginOverlap`
  (params (OverlappedComponent :type "PrimitiveComponent Object Reference") (OtherActor :type "Actor Object Reference") (OtherComp :type "PrimitiveComponent Object Reference") (OtherBodyIndex :type Integer) (bFromSweep :type Boolean) (SweepResult :type "HitResult Structure (by ref)"))
  (if (== OtherActor (`self.Player ref`))
    (`self.EnableInput` (`GameplayStatics.GetPlayerController` 0))
    (set `self.Can_interact` true)))

(event `self.Collision.OnComponentEndOverlap`
  (params (OverlappedComponent :type "PrimitiveComponent Object Reference") (OtherActor :type "Actor Object Reference") (OtherComp :type "PrimitiveComponent Object Reference") (OtherBodyIndex :type Integer))
  (if (== (`self.Player ref`) OtherActor)
    (`self.DisableInput` (`GameplayStatics.GetPlayerController` 0))
    (set `self.Can_interact` false)))

(fn `UserConstructionScript`
  (`parent.UserConstructionScript`))