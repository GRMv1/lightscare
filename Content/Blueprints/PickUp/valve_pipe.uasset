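; Interactable valve that the player turns to shut off every Pipe actor in the level.
; Collision overlap toggles player input and CanInteract, skipping activation once the valve is used.
; Pressing pick_up while it is Hovered and Discovered plays a squeak and a timeline that pitches the Sphere.
; When the turn finishes, it clears ValveOpen on all Pipes, stops the sound and marks itself used.
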(event `self.ReceiveBeginPlay`
  (`parent.ReceiveBeginPlay`)
  (set `self.Discovered` false))

(event `InputAction|pick_up`
  (params (Key :type "Key Structure"))
  (bind _sphere (`self.Sphere`))
  (bind (_relativerotation_roll _relativerotation_pitch _relativerotation_yaw) (`KismetMathLibrary.BreakRotator` (`SceneComponent.RelativeRotation` _sphere)))
  (:`Pressed`
    (if (`self.Hovered`)
      (if (`self.Discovered`)
        (`AudioComponent.Play` (`self.squeaky_valve`) 0.0)
        (bind (_direction _turn) (`Timeline|turn`)
          (:`Update`
            (`SceneComponent.K2_SetRelativeRotation` _sphere (`KismetMathLibrary.MakeRotator` _relativerotation_roll _turn _relativerotation_yaw) false false))
          (:`Finished`
            (bind _outactors (`GameplayStatics.GetAllActorsOfClass` "/Game/Blueprints/przelacznik/pipe.pipe_C"))
            (for _array_element _outactors
              (set `/Game/Blueprints/przelacznik/pipe.valve_open` false _array_element)
              (`AudioComponent.Stop` (`self.squeaky_valve`))
              (set `self.Active` false)
              (set `self.used` true))))))))

(event `self.Collision.OnComponentBeginOverlap`
  (params (OverlappedComponent :type "PrimitiveComponent Object Reference") (OtherActor :type "Actor Object Reference") (OtherComp :type "PrimitiveComponent Object Reference") (OtherBodyIndex :type Integer) (bFromSweep :type Boolean) (SweepResult :type "HitResult Structure (by ref)"))
  (if (== OtherActor (`self.Player ref`))
    (if (`self.used`)
      (set `self.Active` false)
      (else
        (set `self.Can_interact` true)
        (`self.EnableInput` (`GameplayStatics.GetPlayerController` 0))))))

(event `self.Collision.OnComponentEndOverlap`
  (params (OverlappedComponent :type "PrimitiveComponent Object Reference") (OtherActor :type "Actor Object Reference") (OtherComp :type "PrimitiveComponent Object Reference") (OtherBodyIndex :type Integer))
  (if (== (`self.Player ref`) OtherActor)
    (set `self.Can_interact` false)
    (`self.DisableInput` (`GameplayStatics.GetPlayerController` 0))))

(fn `UserConstructionScript`
  (`parent.UserConstructionScript`))