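; Door actor that the player can open once the required number of switches is enabled.
; On Box overlap, it enables input only if AllSwitchPressed equals the length of the character's SwitchWhichEnabled array, and disables input on exit.
; The use action plays or reverses a timeline that yaws the Sphere component and updates ClosedDoor.
; Press-E prompt and endgame-to-MainMenu logic are present but disconnected.
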(event `self.Collision.OnComponentBeginOverlap`
  (params (OverlappedComponent :type "PrimitiveComponent Object Reference") (OtherActor :type "Actor Object Reference") (OtherComp :type "PrimitiveComponent Object Reference") (OtherBodyIndex :type Integer) (bFromSweep :type Boolean) (SweepResult :type "HitResult Structure (by ref)")))

(event `self.Box.OnComponentBeginOverlap`
  (params (OverlappedComponent :type "PrimitiveComponent Object Reference") (OtherActor :type "Actor Object Reference") (OtherComp :type "PrimitiveComponent Object Reference") (OtherBodyIndex :type Integer) (bFromSweep :type Boolean) (SweepResult :type "HitResult Structure (by ref)"))
  (bind _returnvalue (`GameplayStatics.GetPlayerController` 0))
  (if (== OtherActor (`self.Player ref`))
    (set `self.Can_interact` true)
    (bind _asfirst_person_character (cast `/Game/FirstPersonBP/Blueprints/FirstPersonCharacter` OtherActor))
    (if (== (`self.all_switch_pressed`) (`KismetArrayLibrary.Array_Length` (`/Game/FirstPersonBP/Blueprints/FirstPersonCharacter.switch_which_enabled` _asfirst_person_character)))
      (`self.EnableInput` _returnvalue)
      (else
        (`self.DisableInput` _returnvalue :!label _label)))))

(event `self.Box.OnComponentEndOverlap`
  (params (OverlappedComponent :type "PrimitiveComponent Object Reference") (OtherActor :type "Actor Object Reference") (OtherComp :type "PrimitiveComponent Object Reference") (OtherBodyIndex :type Integer))
  (if (== (`self.Player ref`) OtherActor)
    (set `self.Can_interact` false)
    (cast `/Game/FirstPersonBP/Blueprints/FirstPersonCharacter` OtherActor)
    (goto _label)))

(event `self.Collision.OnComponentEndOverlap`
  (params (OverlappedComponent :type "PrimitiveComponent Object Reference") (OtherActor :type "Actor Object Reference") (OtherComp :type "PrimitiveComponent Object Reference") (OtherBodyIndex :type Integer)))

(event `InputAction|use`
  (params (Key :type "Key Structure"))
  (:`Pressed`
    (if (`self.closed_door`)
      (bind (_direction _door_open) (`Timeline|Timeline_0` :!label _label_2)
        (:`Update`
          (`SceneComponent.K2_SetRelativeRotation` (`self.Sphere`) (`KismetMathLibrary.MakeRotator` 0.0 0.0 _door_open) false false)
          (set `self.closed_door` (< _door_open 1.0))))
      (else
        (goto _label_2 :!via `Reverse`)))))

(fn `UserConstructionScript`
  (`parent.UserConstructionScript`))