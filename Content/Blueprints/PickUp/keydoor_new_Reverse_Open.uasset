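; Key-locked door that the player opens and closes with the pick_up input, enabled while they are inside its Box trigger.
; Once Discovered, a press checks the character's DoorItems flag at DoorItemValue.
; Without the key, it plays a locked-handle sound and a hint chosen by SubtitlesId through Text_bot_screen.
; With it, a hovered press plays the door sound and flip-flops a timeline that yaws the Sphere component open or back.
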(event `InputAction|pick_up`
  (params (Key :type "Key Structure"))
  (bind _subtitles_id (`self.subtitles_id`))
  (bind _open_door_2_fast_cue (`self.open_door_2_fast_Cue`))
  (:`Pressed`
    (if (`self.Discovered`)
      (for (_array_element _array_index) (`/Game/FirstPersonBP/Blueprints/FirstPersonCharacter.door_items` (cast `/Game/FirstPersonBP/Blueprints/FirstPersonCharacter` (`GameplayStatics.GetPlayerCharacter` 0) :!pure true))
        (if (and _array_element (== _array_index (`self.door_item_value`)))
          (set `self.need_subtitle` false)))
      (if (`self.need_subtitle`)
        (if (== _subtitles_id 0)
          (`/Engine/EditorBlueprintResources/StandardMacros.DoOnce` (`/Game/FirstPersonBP/Blueprints/GameInstance_new.Was_in_basement` (cast `/Game/FirstPersonBP/Blueprints/GameInstance_new` (`GameplayStatics.GetGameInstance`) :!pure true)) :!label _label
            (:`Completed`
              (`AudioComponent.Play` (`self.Trying-to-Open-Door-Handle-2_Cue`) 0.0)
              (bind _foundwidgets (`WidgetBlueprintLibrary.GetAllWidgetsOfClass` "/Game/HUD/text_bot_screen.text_bot_screen_C"))
              (`/Game/HUD/text_bot_screen.ShowMessage` _foundwidgets "Ah, they're closed. I have probably left keys in my jacket" 5.0)
              (set `self.clicked` true)
              (goto _label :!via `Reset`)))
          (elif (== _subtitles_id 1)
            (`/Engine/EditorBlueprintResources/StandardMacros.DoOnce` false :!label _label_2
              (:`Completed`
                (`AudioComponent.Play` (`self.Trying-to-Open-Door-Handle-2_Cue`) 0.0)
                (bind _foundwidgets_2 (`WidgetBlueprintLibrary.GetAllWidgetsOfClass` "/Game/HUD/text_bot_screen.text_bot_screen_C"))
                (`/Game/HUD/text_bot_screen.ShowMessage` _foundwidgets_2 "Damn, it's closed. If I remember correctly,  \nthe key is hidden in the hunting stand just behing the house " 5.0)
                (goto _label_2 :!via `Reset`)))))
        (elif (`self.Hovered`)
          (`AudioComponent.Stop` _open_door_2_fast_cue)
          (`AudioComponent.Play` _open_door_2_fast_cue 0.0)
          (`/Engine/EditorBlueprintResources/StandardMacros.FlipFlop`
            (:`A`
              (bind (_direction _door_open) (`Timeline|Timeline_0` :!label _label_3)
                (:`Update`
                  (`SceneComponent.K2_SetRelativeRotation` (`self.Sphere`) (`KismetMathLibrary.MakeRotator` 0.0 0.0 _door_open) false false)
                  (set `self.closed_door` (< _door_open 1.0)))
                (:`Finished`
                  (`AudioComponent.Stop` _open_door_2_fast_cue))))
            (:`B`
              (goto _label_3 :!via `Reverse`))))))))

(event `self.Collision.OnComponentBeginOverlap`
  (params (OverlappedComponent :type "PrimitiveComponent Object Reference") (OtherActor :type "Actor Object Reference") (OtherComp :type "PrimitiveComponent Object Reference") (OtherBodyIndex :type Integer) (bFromSweep :type Boolean) (SweepResult :type "HitResult Structure (by ref)")))

(event `self.Box.OnComponentBeginOverlap`
  (params (OverlappedComponent :type "PrimitiveComponent Object Reference") (OtherActor :type "Actor Object Reference") (OtherComp :type "PrimitiveComponent Object Reference") (OtherBodyIndex :type Integer) (bFromSweep :type Boolean) (SweepResult :type "HitResult Structure (by ref)"))
  (if (== OtherActor (cast `/Game/FirstPersonBP/Blueprints/FirstPersonCharacter` (`GameplayStatics.GetPlayerCharacter` 0) :!pure true))
    (`self.EnableInput` (`GameplayStatics.GetPlayerController` 0))
    (set `self.Can_interact` true)))

(event `self.Box.OnComponentEndOverlap`
  (params (OverlappedComponent :type "PrimitiveComponent Object Reference") (OtherActor :type "Actor Object Reference") (OtherComp :type "PrimitiveComponent Object Reference") (OtherBodyIndex :type Integer))
  (if (== (cast `/Game/FirstPersonBP/Blueprints/FirstPersonCharacter` (`GameplayStatics.GetPlayerCharacter` 0) :!pure true) OtherActor)
    (`self.DisableInput` (`GameplayStatics.GetPlayerController` 0))
    (set `self.Can_interact` false)))

(event `self.Collision.OnComponentEndOverlap`
  (params (OverlappedComponent :type "PrimitiveComponent Object Reference") (OtherActor :type "Actor Object Reference") (OtherComp :type "PrimitiveComponent Object Reference") (OtherBodyIndex :type Integer)))

(fn `UserConstructionScript`
  (`parent.UserConstructionScript`))