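; Coat is an interactable that plays a rustling sound and shows a hint that the keys may be in a kitchen drawer.
; Collision overlap sets Active from the Cabinet's Completed state and whether a Keydoor_new_2 was clicked, enabling input for the player when active.
; The pick_up action responds only when Hovered and Discovered, sets WasClicked, and immediately resets its DoOnce, so it can repeat.
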(event `self.ReceiveBeginPlay`
  (`parent.ReceiveBeginPlay`)
  (set `self.Discovered` false))

(event `InputAction|pick_up`
  (params (Key :type "Key Structure"))
  (:`Pressed`
    (if (`self.Hovered`)
      (if (`self.Discovered`)
        (`/Engine/EditorBlueprintResources/StandardMacros.DoOnce` false :!label _label
          (:`Completed`
            (set `self.was_clicked` true)
            (`GameplayStatics.PlaySoundAtLocation` "/Game/Audio/Latarka/szuranie2_cichsze.szuranie2_cichsze" (`SceneComponent.RelativeLocation` (`self.Sphere`)) (struct) 1.0 1.0 0.0 null null null)
            (bind _foundwidgets (`WidgetBlueprintLibrary.GetAllWidgetsOfClass` "/Game/HUD/text_bot_screen.text_bot_screen_C"))
            (`/Game/HUD/text_bot_screen.ShowMessage` _foundwidgets "Umm, maybe the keys are in a kitchen drawer" 3.0)
            (goto _label :!via `Reset`)))))))

(event `self.Collision.OnComponentBeginOverlap`
  (params (OverlappedComponent :type "PrimitiveComponent Object Reference") (OtherActor :type "Actor Object Reference") (OtherComp :type "PrimitiveComponent Object Reference") (OtherBodyIndex :type Integer) (bFromSweep :type Boolean) (SweepResult :type "HitResult Structure (by ref)"))
  (bind _returnvalue (`GameplayStatics.GetActorOfClass` "/Game/Blueprints/PickUp/cabinet.cabinet_C"))
  (if (`/Game/Blueprints/PickUp/cabinet.completed` _returnvalue)
    (set `self.Active` false)
    (else
      (bind _outactors (`GameplayStatics.GetAllActorsOfClass` "/Game/Blueprints/PickUp/keydoor_new_2.keydoor_new_2_C"))
      (for _array_element _outactors :!label _label_2
        (if (`/Game/Blueprints/PickUp/keydoor_new_2.clicked` _array_element)
          (if (`self.was_clicked`)
            _
            (else
              _))
          (set `self.Active` true)
          (if (== OtherActor (cast `/Game/FirstPersonBP/Blueprints/FirstPersonCharacter` (`GameplayStatics.GetPlayerCharacter` 0) :!pure true))
            (set `self.Can_interact` true)
            (`self.EnableInput` (`GameplayStatics.GetPlayerController` 0))
            (break))
          (else
            (set `self.Active` false)))))))

(event `self.Collision.OnComponentEndOverlap`
  (params (OverlappedComponent :type "PrimitiveComponent Object Reference") (OtherActor :type "Actor Object Reference") (OtherComp :type "PrimitiveComponent Object Reference") (OtherBodyIndex :type Integer))
  (if (== (cast `/Game/FirstPersonBP/Blueprints/FirstPersonCharacter` (`GameplayStatics.GetPlayerCharacter` 0) :!pure true) OtherActor)
    (set `self.Can_interact` false)
    (`self.DisableInput` (`GameplayStatics.GetPlayerController` 0))
    (goto _label_2 :!via `Break`)))

(fn `UserConstructionScript`
  (`parent.UserConstructionScript`))