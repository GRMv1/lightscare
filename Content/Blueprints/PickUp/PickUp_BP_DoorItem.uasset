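; Door item pickup actor that the player collects into the first-person character's inventory.
; Collision overlap toggles input and interactability, so pressing pick_up while in range and hovered triggers a one-time pickup.
; Pickup inserts true into the character's DoorItems at DoorItemValue, adds a "doorItem" inventory entry and plays a sound.
; It hides the sphere, shows a Pickup_key widget for two seconds, flags the character's IsDestroyedPickupItem and destroys itself.
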(event `self.PickUp`)

(event `InputAction|pick_up`
  (params (Key :type "Key Structure"))
  (:`Pressed`
    (if (and (`self.Can_interact`) (`self.Hovered`))
      (`/Engine/EditorBlueprintResources/StandardMacros.DoOnce` false
        (:`Completed`
          (bind _asfirst_person_character (cast `/Game/FirstPersonBP/Blueprints/FirstPersonCharacter` (`GameplayStatics.GetPlayerCharacter` 0)))
          (`KismetArrayLibrary.Array_Insert` (`/Game/FirstPersonBP/Blueprints/FirstPersonCharacter.door_items` _asfirst_person_character) true (`self.door_item_value`))
          (`/Game/FirstPersonBP/Blueprints/FirstPersonCharacter.addInventoryItem` _asfirst_person_character "doorItem")
          (`GameplayStatics.PlaySoundAtLocation` "/Game/Audio/Latarka/szuranie1_ciszej.szuranie1_ciszej" (`SceneComponent.RelativeLocation` (`self.Sphere`)) (struct) 1.0 1.0 0.0 null null null)
          (bind _returnvalue (`|CreateWidget` "/Game/HUD/pickup_key.pickup_key_C"))
          (`UserWidget.AddToViewport` _returnvalue 0)
          (`self.DisableInput` (`GameplayStatics.GetPlayerController` 0))
          (`SceneComponent.SetVisibility` (`self.Sphere`) false false)
          (`KismetSystemLibrary.Delay` 2.0)
          (`Widget.RemoveFromParent` _returnvalue)
          (set `/Game/FirstPersonBP/Blueprints/FirstPersonCharacter.is_destroyed_pickup_item` true _asfirst_person_character)
          (`self.K2_DestroyActor`))))))

(event `self.Collision.OnComponentBeginOverlap`
  (params (OverlappedComponent :type "PrimitiveComponent Object Reference") (OtherActor :type "Actor Object Reference") (OtherComp :type "PrimitiveComponent Object Reference") (OtherBodyIndex :type Integer) (bFromSweep :type Boolean) (SweepResult :type "HitResult Structure (by ref)"))
  (if (== OtherActor (`self.Player ref`))
    (set `self.Can_interact` true)
    (`self.EnableInput` (`GameplayStatics.GetPlayerController` 0))))

(event `self.Collision.OnComponentEndOverlap`
  (params (OverlappedComponent :type "PrimitiveComponent Object Reference") (OtherActor :type "Actor Object Reference") (OtherComp :type "PrimitiveComponent Object Reference") (OtherBodyIndex :type Integer))
  (if (== (`self.Player ref`) OtherActor)
    (set `self.Can_interact` false)
    (`self.DisableInput` (`GameplayStatics.GetPlayerController` 0))))

(fn `UserConstructionScript`
  (`parent.UserConstructionScript`))