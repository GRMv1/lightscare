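; Interactive drawer actor (szuflada) that the player slides open and closed with the "use" input.
; On use, a short multi-object line trace from the first-person camera takes the first hit static mesh component and checks it is named "szuflada".
; Its relative X position picks opening or closing, and one of two timelines lerps it by SlideLength with a drawer sound.
; CanOpen blocks re-triggering during movement.
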(event `self.ReceiveBeginPlay`
  (`parent.ReceiveBeginPlay`)
  (`self.EnableInput` (`GameplayStatics.GetPlayerController` 0)))

(event `InputAction|use`
  (params (Key :type "Key Structure"))
  (bind _returnvalue (`self.K2_GetActorLocation`))
  (bind (_relativelocation_x _relativelocation_y _relativelocation_z) (`KismetMathLibrary.BreakVector` (`SceneComponent.RelativeLocation` (`self.StaticMesh REF`))))
  (bind (_relativelocation_x_2 _relativelocation_y_2 _relativelocation_z_2) (`KismetMathLibrary.BreakVector` (`SceneComponent.RelativeLocation` (`self.StaticMesh REF`))))
  (:`Pressed`
    (if (`self.CanOpen`)
      (set `self.CanOpen` false)
      (bind _asfirst_person_character (cast `/Game/FirstPersonBP/Blueprints/FirstPersonCharacter` (`GameplayStatics.GetPlayerCharacter` 0))
        (:`then`
          (bind _firstpersoncamera (`/Game/FirstPersonBP/Blueprints/FirstPersonCharacter.FirstPersonCamera` _asfirst_person_character))
          (bind _returnvalue_2 (`SceneComponent.K2_GetComponentLocation` _firstpersoncamera))
          (bind _outhits (`KismetSystemLibrary.LineTraceMultiForObjects` :`Start` _returnvalue_2 :`End` (+ (* (`SceneComponent.GetForwardVector` _firstpersoncamera) 150.0) _returnvalue_2) :`ObjectTypes` (`|MakeArray` "ObjectTypeQuery2" :!type "EObjectTypeQuery Enum") :`bIgnoreSelf` false))
          (for _array_element _outhits
            (bind _asstatic_mesh_component (cast `StaticMeshComponent` (`.HitComponent` (`GameplayStatics.BreakHitResult` _array_element))))
            (break))
          (if (`KismetStringLibrary.EqualEqual_StrStr` (`KismetSystemLibrary.GetObjectName` _asstatic_mesh_component) "szuflada")
            (set `self.StaticMesh REF` _asstatic_mesh_component)
            (bind _relativelocation_x_3 (`KismetMathLibrary.BreakVector` (`SceneComponent.RelativeLocation` _asstatic_mesh_component)))
            (if (not (>= _relativelocation_x_3 (- (`self.SlideLength`) 1.0)))
              (`GameplayStatics.PlaySoundAtLocation` "/Game/Audio/cabinet/drawer_sound_cue.drawer_sound_cue" _returnvalue (struct) 1.0 1.0 0.0 null null null)
              (set `self.StartLoc` (`KismetMathLibrary.MakeVector` _relativelocation_x _relativelocation_y _relativelocation_z))
              (set `self.EndLoc` (`KismetMathLibrary.MakeVector` (+ _relativelocation_x (`self.SlideLength`)) _relativelocation_y _relativelocation_z))
              (bind (_direction _newtrack_0) (`Timeline|Timeline_0` :!via `PlayFromStart`)
                (:`Update`
                  (bind _returnvalue_3 (`KismetMathLibrary.VLerp` (`self.StartLoc`) (`self.EndLoc`) _newtrack_0))
                  (`SceneComponent.K2_SetRelativeLocation` (`self.StaticMesh REF`) _returnvalue_3 false false))
                (:`Finished`
                  (set `self.CanOpen` true)
                  (`KismetSystemLibrary.PrintString` (`KismetStringLibrary.Conv_VectorToString` _returnvalue_3))))
              (else
                (`GameplayStatics.PlaySoundAtLocation` "/Game/Audio/cabinet/drawer_sound_cue.drawer_sound_cue" _returnvalue (struct) 1.0 1.0 0.0 null null null)
                (set `self.StartLoc` (`KismetMathLibrary.MakeVector` _relativelocation_x_2 _relativelocation_y_2 _relativelocation_z_2))
                (set `self.EndLoc` (`KismetMathLibrary.MakeVector` (+ _relativelocation_x_2 (* -1 (`self.SlideLength`))) _relativelocation_y_2 _relativelocation_z_2))
                (bind (_direction_2 _newtrack_0_2) (`Timeline|Timeline_1` :!via `PlayFromStart`)
                  (:`Update`
                    (`SceneComponent.K2_SetRelativeLocation` (`self.StaticMesh REF`) (`KismetMathLibrary.VLerp` (`self.StartLoc`) (`self.EndLoc`) _newtrack_0_2) false false))
                  (:`Finished`
                    (set `self.CanOpen` true)))))
            (else
              (set `self.CanOpen` true))))
        (:`CastFailed`
          (`KismetSystemLibrary.PrintString` "first per cast fail"))))))

(fn `UserConstructionScript`
  (`parent.UserConstructionScript`))