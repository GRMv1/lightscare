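; PickUp_BP_DoorItem3 is a pickup actor that grants the player a door item.
; Its PickUp event runs once, casts player 0 to FirstPersonCharacter and inserts true into that character's DoorItems array at the DoorItemValue index.
; The actor then destroys itself; BeginPlay, Tick and overlap events are disabled stubs, so collection depends on PickUp being triggered.
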(event `self.PickUp`
  (`/Engine/EditorBlueprintResources/StandardMacros.DoOnce` false
    (:`Completed`
      (bind _asfirst_person_character (cast `/Game/FirstPersonBP/Blueprints/FirstPersonCharacter` (`GameplayStatics.GetPlayerCharacter` 0)))
      (`KismetArrayLibrary.Array_Insert` (`/Game/FirstPersonBP/Blueprints/FirstPersonCharacter.door_items` _asfirst_person_character) true (`self.door_item_value`))
      (`self.K2_DestroyActor`))))

(fn `UserConstructionScript`
  (`parent.UserConstructionScript`))