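; Car door interactable that swings open on the pick_up input once the player has the car key.
; Collision overlap toggles input and CanInteract; with the key, a hovered, closed door plays audio and a yaw timeline, then destroys its collision and deactivates.
; Without the key, input shows a temporary INeedKeys widget, regardless of hover.
; An already-open door reverses the timeline.
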(event `self.ReceiveBeginPlay`
  (`parent.ReceiveBeginPlay`))

(event `InputAction|pick_up`
  (params (Key :type "Key Structure"))
  (:`Pressed`
    (if (`/Game/FirstPersonBP/Blueprints/FirstPersonCharacter.has_car_key` (`self.Player ref`))
      (if (and (`self.Hovered`) (`self.Can_interact`))
        (if (`self.Closed_Door`)
          (`AudioComponent.Play` (`self.Audio`) 0.0)
          (bind (_direction _door_open) (`Timeline|Timeline_0` :!label _label)
            (:`Update`
              (`SceneComponent.K2_SetRelativeRotation` (`self.DefaultSceneRoot`) (`KismetMathLibrary.MakeRotator` 0.0 0.0 _door_open) false false))
            (:`Finished`
              (`ActorComponent.K2_DestroyComponent` (`self.Collision`))
              (set `self.Closed_Door` false)
              (set `self.Active` false)))
          (else
            (goto _label :!via `Reverse`))))
      (else
        (bind _returnvalue (`|CreateWidget` "/Game/HUD/Subtitles/INeedKeys.INeedKeys_C"))
        (`UserWidget.AddToViewport` _returnvalue 0)
        (`KismetSystemLibrary.Delay` 3.0)
        (`Widget.RemoveFromParent` _returnvalue)))))

(event `self.Collision.OnComponentBeginOverlap`
  (params (OverlappedComponent :type "PrimitiveComponent Object Reference") (OtherActor :type "Actor Object Reference") (OtherComp :type "PrimitiveComponent Object Reference") (OtherBodyIndex :type Integer) (bFromSweep :type Boolean) (SweepResult :type "HitResult Structure (by ref)"))
  (if (== OtherActor (`self.Player ref`))
    (`self.EnableInput` (`GameplayStatics.GetPlayerController` 0))
    (set `self.Can_interact` true)))

(event `self.Collision.OnComponentEndOverlap`
  (params (OverlappedComponent :type "PrimitiveComponent Object Reference") (OtherActor :type "Actor Object Reference") (OtherComp :type "PrimitiveComponent Object Reference") (OtherBodyIndex :type Integer))
  (if (== (`self.Player ref`) OtherActor)
    (`self.DisableInput` (`GameplayStatics.GetPlayerController` 0))
    (set `self.Can_interact` false)))

(fn `UserConstructionScript`
  (`parent.UserConstructionScript`))