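; Interactable phone that drives two story calls, chosen by the GameInstance's WasInBasement flag.
; It rings on BeginPlay before the basement visit; overlap events toggle player input and, after the basement, reactivate it with a larger collision sphere.
; Pressing pick_up while hovered either fires the first cutscene dispatcher, or clears the flag, shows a police greeting and fires the last-call dispatcher.
; Older inline dialogue and camera tests remain unconnected.
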(event `self.ReceiveBeginPlay`
  (set `self.Discovered` true)
  (bind _asgame_instance_new (cast `/Game/FirstPersonBP/Blueprints/GameInstance_new` (`GameplayStatics.GetGameInstance`)))
  (if (not (`/Game/FirstPersonBP/Blueprints/GameInstance_new.Was_in_basement` _asgame_instance_new))
    (`AudioComponent.Play` (`self.ringing`) 0.0)))

(event `InputAction|pick_up`
  (params (Key :type "Key Structure"))
  (:`Pressed`
    (if (`self.Hovered`)
      (bind _asgame_instance_new (cast `/Game/FirstPersonBP/Blueprints/GameInstance_new` (`GameplayStatics.GetGameInstance`)))
      (if (`/Game/FirstPersonBP/Blueprints/GameInstance_new.Was_in_basement` _asgame_instance_new)
        (`/Engine/EditorBlueprintResources/StandardMacros.DoOnce` false
          (:`Completed`
            (set `/Game/FirstPersonBP/Blueprints/GameInstance_new.Was_in_basement` false (cast `/Game/FirstPersonBP/Blueprints/GameInstance_new` (`GameplayStatics.GetGameInstance`) :!pure true))
            (`AudioComponent.Play` (`self.pickup_phone`) 0.0)
            (bind _foundwidgets (`WidgetBlueprintLibrary.GetAllWidgetsOfClass` "/Game/HUD/text_bot_screen.text_bot_screen_C"))
            (`/Game/HUD/text_bot_screen.ShowMessage` :`self` _foundwidgets :`text` "Police Officer: Hello, what's your emergency?" :`time` 2.0)
            (`self.LastPhoneCallDispatcher`)))
        (else
          (`/Engine/EditorBlueprintResources/StandardMacros.DoOnce` false
            (:`Completed`
              (`AudioComponent.Stop` (`self.ringing`))
              (`AudioComponent.Play` (`self.pickup_phone`) 0.0)
              (`self.FirstCutsceneDispatcher`)
              (`self.DisableInput` null)
              (set `self.Active` false)
              (set `self.first_call_passed` true))))))))

(event `self.Collision.OnComponentBeginOverlap`
  (params (OverlappedComponent :type "PrimitiveComponent Object Reference") (OtherActor :type "Actor Object Reference") (OtherComp :type "PrimitiveComponent Object Reference") (OtherBodyIndex :type Integer) (bFromSweep :type Boolean) (SweepResult :type "HitResult Structure (by ref)"))
  (bind _asgame_instance_new (cast `/Game/FirstPersonBP/Blueprints/GameInstance_new` (`GameplayStatics.GetGameInstance`)))
  (if (`/Game/FirstPersonBP/Blueprints/GameInstance_new.Was_in_basement` _asgame_instance_new)
    (`SphereComponent.SetSphereRadius` (`self.Collision`) 500.0 true)
    (set `self.Active` true))
  (if (== OtherActor (cast `/Game/FirstPersonBP/Blueprints/FirstPersonCharacter` (`GameplayStatics.GetPlayerCharacter` 0) :!pure true))
    (set `self.Can_interact` true)
    (`self.EnableInput` (`GameplayStatics.GetPlayerController` 0))))

(event `self.Collision.OnComponentEndOverlap`
  (params (OverlappedComponent :type "PrimitiveComponent Object Reference") (OtherActor :type "Actor Object Reference") (OtherComp :type "PrimitiveComponent Object Reference") (OtherBodyIndex :type Integer))
  (if (== (cast `/Game/FirstPersonBP/Blueprints/FirstPersonCharacter` (`GameplayStatics.GetPlayerCharacter` 0) :!pure true) OtherActor)
    (set `self.Can_interact` false)
    (`self.DisableInput` (`GameplayStatics.GetPlayerController` 0))))

(fn `UserConstructionScript`
  (`parent.UserConstructionScript`))