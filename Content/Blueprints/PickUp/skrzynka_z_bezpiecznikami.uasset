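; Fuse box pickup-interaction actor where a player carrying a fuse (bezpiecznik) repairs broken switches, once only.
; The collision volume enables the actor's input while the player overlaps it, so pick_up works only nearby.
; If the player has a fuse, the hidden fuse component becomes visible and every Broken_switch_bezpiecznik is marked unbroken.
; It also calls SwitchLightRedOrYellowBezpiecznik on every Switch_light_broken to update their lights.
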(event `self.ReceiveBeginPlay`
  (`parent.ReceiveBeginPlay`)
  (`SceneComponent.SetVisibility` (`self.bezpiecznik`) false false))

(event `InputAction|pick_up`
  (params (Key :type "Key Structure"))
  (:`Pressed`
    (if (not (`self.was_used`))
      (bind _asfirst_person_character (cast `/Game/FirstPersonBP/Blueprints/FirstPersonCharacter` (`GameplayStatics.GetPlayerCharacter` 0)))
      (if (`/Game/FirstPersonBP/Blueprints/FirstPersonCharacter.has_bezpiecznik` _asfirst_person_character)
        (`SceneComponent.SetVisibility` (`self.bezpiecznik`) true false)
        (bind _outactors (`GameplayStatics.GetAllActorsOfClass` "/Game/Blueprints/PickUp/broken_switch_bezpiecznik.broken_switch_bezpiecznik_C"))
        (for _array_element _outactors
          (set `/Game/Blueprints/PickUp/broken_switch_bezpiecznik.is_broken` false _array_element))
        (set `self.was_used` true)
        (bind _outactors_2 (`GameplayStatics.GetAllActorsOfClass` "/Game/Blueprints/przelacznik/switch_light_broken.switch_light_broken_C"))
        (for _array_element_2 _outactors_2
          (`/Game/Blueprints/przelacznik/switch_light_broken.SwitchLightRedOrYellowBezpiecznik` _array_element_2))))))

(event `self.Collision.OnComponentBeginOverlap`
  (params (OverlappedComponent :type "PrimitiveComponent Object Reference") (OtherActor :type "Actor Object Reference") (OtherComp :type "PrimitiveComponent Object Reference") (OtherBodyIndex :type Integer) (bFromSweep :type Boolean) (SweepResult :type "HitResult Structure (by ref)"))
  (if (== OtherActor (cast `/Game/FirstPersonBP/Blueprints/FirstPersonCharacter` (`GameplayStatics.GetPlayerCharacter` 0) :!pure true))
    (set `self.Can_interact` true)
    (`self.EnableInput` (`GameplayStatics.GetPlayerController` 0))))

(event `self.Collision.OnComponentEndOverlap`
  (params (OverlappedComponent :type "PrimitiveComponent Object Reference") (OtherActor :type "Actor Object Reference") (OtherComp :type "PrimitiveComponent Object Reference") (OtherBodyIndex :type Integer))
  (if (== (cast `/Game/FirstPersonBP/Blueprints/FirstPersonCharacter` (`GameplayStatics.GetPlayerCharacter` 0) :!pure true) OtherActor)
    (set `self.Can_interact` false)
    (`self.DisableInput` (`GameplayStatics.GetPlayerController` 0))))

(fn `UserConstructionScript`
  (`parent.UserConstructionScript`))