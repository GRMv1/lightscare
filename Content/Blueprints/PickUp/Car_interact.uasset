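; Interactable car actor that lets the player toggle its left and right lights on and off with a sound.
; The pick_up input works only while the actor is hovered and the player is inside the collision sphere, whose overlaps also enable and disable input.
; Tick looks up the Car_door actor every frame and enlarges the sphere while that door is open, with no path to shrink it back.
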(event `InputAction|pick_up`
  (params (Key :type "Key Structure"))
  (:`Pressed`
    (if (and (`self.Hovered`) (`self.Can_interact`))
      (`AudioComponent.Play` (`self.Audio`) 0.0)
      (if (`self.Light_is_on`)
        (`SceneComponent.SetVisibility` (`self.L`) false false)
        (`SceneComponent.SetVisibility` (`self.R`) false false)
        (set `self.Light_is_on` false)
        (else
          (`SceneComponent.SetVisibility` (`self.L`) true false)
          (`SceneComponent.SetVisibility` (`self.R`) true false)
          (set `self.Light_is_on` true))))))

(event `self.ReceiveTick`
  (params (DeltaSeconds :type "Float (single-precision)"))
  (`parent.ReceiveTick` DeltaSeconds)
  (bind _returnvalue (`GameplayStatics.GetActorOfClass` "/Game/Blueprints/PickUp/Car_door.Car_door_C"))
  (if (not (`/Game/Blueprints/PickUp/Car_door.Closed_Door` _returnvalue))
    (`SphereComponent.SetSphereRadius` (`self.Collision`) 304.0 true)))

(event `self.Collision.OnComponentBeginOverlap`
  (params (OverlappedComponent :type "PrimitiveComponent Object Reference") (OtherActor :type "Actor Object Reference") (OtherComp :type "PrimitiveComponent Object Reference") (OtherBodyIndex :type Integer) (bFromSweep :type Boolean) (SweepResult :type "HitResult Structure (by ref)"))
  (if (== OtherActor (`self.Player ref`))
    (set `self.Can_interact` true)
    (`self.EnableInput` (`GameplayStatics.GetPlayerController` 0))))

(event `self.Collision.OnComponentEndOverlap`
  (params (OverlappedComponent :type "PrimitiveComponent Object Reference") (OtherActor :type "Actor Object Reference") (OtherComp :type "PrimitiveComponent Object Reference") (OtherBodyIndex :type Integer))
  (if (== (`self.Player ref`) OtherActor)
    (set `self.Can_interact` false)
    (`self.DisableInput` (`GameplayStatics.GetPlayerController` 0))))

(fn `UserConstructionScript`
  (`parent.UserConstructionScript`))