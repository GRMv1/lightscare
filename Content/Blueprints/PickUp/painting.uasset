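; Interactive painting actor that shifts its Sphere component once, with a sound, when the player uses it.
; Box overlaps with PlayerRef toggle CanInteract and the actor's input, though the use event never checks that flag.
; A DoOnce-gated press plays a sound at the Sphere's relative location and starts timelines X, Z and Rotacja, chained through Update pins, with the last setting relative location and animated pitch.
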(event `self.Box.OnComponentBeginOverlap`
  (params (OverlappedComponent :type "PrimitiveComponent Object Reference") (OtherActor :type "Actor Object Reference") (OtherComp :type "PrimitiveComponent Object Reference") (OtherBodyIndex :type Integer) (bFromSweep :type Boolean) (SweepResult :type "HitResult Structure (by ref)"))
  (if (== OtherActor (`self.Player ref`))
    (set `self.Can_interact` true)
    (`self.EnableInput` (`GameplayStatics.GetPlayerController` 0))))

(event `self.Box.OnComponentEndOverlap`
  (params (OverlappedComponent :type "PrimitiveComponent Object Reference") (OtherActor :type "Actor Object Reference") (OtherComp :type "PrimitiveComponent Object Reference") (OtherBodyIndex :type Integer))
  (if (== (`self.Player ref`) OtherActor)
    (set `self.Can_interact` false)
    (`self.DisableInput` (`GameplayStatics.GetPlayerController` 0))))

(event `InputAction|use`
  (params (Key :type "Key Structure"))
  (:`Pressed`
    (`/Engine/EditorBlueprintResources/StandardMacros.DoOnce` false
      (:`Completed`
        (`GameplayStatics.SpawnSoundAtLocation` "/Game/Audio/Latarka/szuranie1_ciszej.szuranie1_ciszej" (`SceneComponent.RelativeLocation` (`self.Sphere`)) (struct) 1.0 1.0 0.0 null null)
        (`Timeline|x`
          (:`Update`
            (`Timeline|z`
              (:`Update`
                (bind (_direction _newtrack_0) (`Timeline|rotacja`)
                  (:`Update`
                    (`SceneComponent.K2_SetRelativeLocation` (`self.Sphere`) (0.0 0.0 0.0) false false)
                    (`SceneComponent.K2_SetRelativeRotation` (`self.Sphere`) (`KismetMathLibrary.MakeRotator` 540.0 _newtrack_0 180.0) false false)))))))))))

(fn `UserConstructionScript`
  (`parent.UserConstructionScript`))