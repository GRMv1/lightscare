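; A one-shot wall or world switch that the player activates with the pick_up input to switch the level's lights.
; Collision overlap enables input until the switch is used, while Tick shows or removes a PressE widget based on Hovered.
; Pressing plays a sound, appends an entry to FirstPersonCharacter's SwitchWhichEnabled array, calls SwitchLight on every Switch_light actor and slides the handle along Z with a timeline.
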(event `self.Collision.OnComponentBeginOverlap`
  (params (OverlappedComponent :type "PrimitiveComponent Object Reference") (OtherActor :type "Actor Object Reference") (OtherComp :type "PrimitiveComponent Object Reference") (OtherBodyIndex :type Integer) (bFromSweep :type Boolean) (SweepResult :type "HitResult Structure (by ref)"))
  (bind _returnvalue (`GameplayStatics.GetPlayerController` 0))
  (if (== OtherActor (`self.Player ref`))
    (if (`self.switch_enabled`)
      (set `self.Can_interact` false :!label _label)
      (`self.DisableInput` _returnvalue)
      (else
        (set `self.Can_interact` true)
        (`self.EnableInput` _returnvalue)))))

(event `self.Collision.OnComponentEndOverlap`
  (params (OverlappedComponent :type "PrimitiveComponent Object Reference") (OtherActor :type "Actor Object Reference") (OtherComp :type "PrimitiveComponent Object Reference") (OtherBodyIndex :type Integer))
  (if (== (`self.Player ref`) OtherActor)
    (goto _label)))

(event `self.ReceiveTick`
  (params (DeltaSeconds :type "Float (single-precision)"))
  (if (`self.Hovered`)
    (if (not (`self.is_widget`))
      (bind _returnvalue (`|CreateWidget` "/Game/HUD/PressE.PressE_C" (`GameplayStatics.GetPlayerController` 0)))
      (set `self.is_widget` true)
      (`UserWidget.AddToViewport` _returnvalue 0))
    (elif (`self.is_widget`)
      (`Widget.RemoveFromParent` _returnvalue)
      (set `self.is_widget` false))))

(event `InputAction|pick_up`
  (params (Key :type "Key Structure"))
  (bind (_relativelocation_x _relativelocation_y) (`KismetMathLibrary.BreakVector` (`SceneComponent.RelativeLocation` (`self.switch_handle`))))
  (:`Pressed`
    (`/Engine/EditorBlueprintResources/StandardMacros.DoOnce` false
      (:`Completed`
        (bind _asfirst_person_character (cast `/Game/FirstPersonBP/Blueprints/FirstPersonCharacter` (`GameplayStatics.GetPlayerCharacter` 0)))
        (bind _switch_which_enabled (`/Game/FirstPersonBP/Blueprints/FirstPersonCharacter.switch_which_enabled` _asfirst_person_character))
        (`KismetArrayLibrary.Array_Add` _switch_which_enabled)
        (set `self.switch_enabled` true)
        (`GameplayStatics.PlaySoundAtLocation` "/Game/Audio/przelacznik/switch.switch" (`SceneComponent.RelativeLocation` (`self.Sphere`)) (struct) 1.0 1.0 0.0 null null null)
        (bind _outactors (`GameplayStatics.GetAllActorsOfClass` "/Game/Blueprints/przelacznik/switch_light.switch_light_C"))
        (for _array_element _outactors
          (`/Game/Blueprints/przelacznik/switch_light.SwitchLight` _array_element)
          (for _array_element_2 _switch_which_enabled
            (`KismetSystemLibrary.PrintString` (`KismetStringLibrary.Conv_BoolToString` _array_element_2))
            (bind (_direction _switched) (`Timeline|Timeline_0`)
              (:`Update`
                (`SceneComponent.K2_SetRelativeLocation` (`self.switch_handle`) (`KismetMathLibrary.MakeVector` _relativelocation_x _relativelocation_y _switched) false false)))))))))

(fn `UserConstructionScript`
  (`parent.UserConstructionScript`))