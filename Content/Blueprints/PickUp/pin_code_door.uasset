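; Door actor that the player opens by entering a pin code.
; Its collision overlap toggles nearby state and player input, letting the use action create a pin code widget, pass it the door's code, stop character movement and show the cursor.
; The widget calls back to re-arm the prompt or open the door once, playing audio and a timeline that yaws the Sphere component and closes the overlap gates.
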(event `self.Collision.OnComponentBeginOverlap`
  (params (OverlappedComponent :type "PrimitiveComponent Object Reference") (OtherActor :type "Actor Object Reference") (OtherComp :type "PrimitiveComponent Object Reference") (OtherBodyIndex :type Integer) (bFromSweep :type Boolean) (SweepResult :type "HitResult Structure (by ref)"))
  (if (== OtherActor (`self.Player ref`))
    (set `self.Can_interact` true)
    (cast `/Game/FirstPersonBP/Blueprints/FirstPersonCharacter` OtherActor)
    (`/Engine/EditorBlueprintResources/StandardMacros.Gate` false :!label _label
      (:`Exit`
        (set `self.near` true)
        (`self.EnableInput` (`GameplayStatics.GetPlayerController` 0))))))

(event `self.Collision.OnComponentEndOverlap`
  (params (OverlappedComponent :type "PrimitiveComponent Object Reference") (OtherActor :type "Actor Object Reference") (OtherComp :type "PrimitiveComponent Object Reference") (OtherBodyIndex :type Integer))
  (if (== (`self.Player ref`) OtherActor)
    (set `self.Can_interact` false)
    (cast `/Game/FirstPersonBP/Blueprints/FirstPersonCharacter` OtherActor)
    (`/Engine/EditorBlueprintResources/StandardMacros.Gate` false :!label _label_2
      (:`Exit`
        (set `self.near` false)
        (`self.DisableInput` (`GameplayStatics.GetPlayerController` 0))))))

(event `InputAction|use`
  (params (Key :type "Key Structure"))
  (bind _returnvalue (`GameplayStatics.GetPlayerController` 0))
  (:`Pressed`
    (if (`self.near`)
      (`/Engine/EditorBlueprintResources/StandardMacros.DoOnce` false :!label _label_3
        (:`Completed`
          (bind _returnvalue_2 (`|CreateWidget` "/Game/Blueprints/pin_code_widget.pin_code_widget_C"))
          (`UserWidget.AddToViewport` _returnvalue_2 0)
          (add `/Game/Blueprints/pin_code_widget.Reset` _returnvalue_2 (delegate `reset`))
          (add `/Game/Blueprints/pin_code_widget.OpenDoor` _returnvalue_2 (delegate `opendoor`))
          (set `/Game/Blueprints/pin_code_widget.PinCode` (`self.PinCode`) _returnvalue_2)
          (bind _outactors (`GameplayStatics.GetAllActorsOfClass` "/Game/FirstPersonBP/Blueprints/FirstPersonCharacter.FirstPersonCharacter_C"))
          (set `/Game/FirstPersonBP/Blueprints/FirstPersonCharacter.CanMove` false (`|GetArrayItem` _outactors))
          (set `PlayerController.bShowMouseCursor` true _returnvalue)
          (`Widget.SetUserFocus` _returnvalue_2 _returnvalue))))))

(event `reset`
  (goto _label_3 :!via `Reset`))

(event `opendoor`
  (`/Engine/EditorBlueprintResources/StandardMacros.DoOnce` false
    (:`Completed`
      (`AudioComponent.Play` (`self.Audio`) 0.0)
      (bind (_direction _move) (`Timeline|Timeline_0`)
        (:`Update`
          (`SceneComponent.K2_SetRelativeRotation` (`self.Sphere`) (`KismetMathLibrary.MakeRotator` 0.0 0.0 _move) false false)
          (`|ExecutionSequence`
            (:`then_0`
              (goto _label :!via `Close`))
            (:`then_1`
              (goto _label_2 :!via `Close`))))))))

(fn `UserConstructionScript`
  (`parent.UserConstructionScript`))