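; Interactive cabinet drawer that slides open once to make a door item available for pickup.
; Overlap enables player input only after Kitchen_cabinet has been clicked and while this drawer is unclicked.
; Pressing pick_up while hovered and discovered plays a sound and a timeline sliding Sphere and the child item along Y.
; The item's collision radius is zero until the slide finishes, when input is disabled and "Got it!" appears.
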(event `self.ReceiveBeginPlay`
  (`parent.ReceiveBeginPlay`)
  (set `self.Discovered` false)
  (bind _aspick_up_bp_door_item (cast `/Game/Blueprints/PickUp/PickUp_BP_DoorItem` (`ChildActorComponent.ChildActor` (`self.PickUp_BP_DoorItem`))))
  (`SphereComponent.SetSphereRadius` (`/Game/Blueprints/PickUp/PickUp_BP.Collision` _aspick_up_bp_door_item) 0.0 true))

(event `self.ReceiveTick`
  (params (DeltaSeconds :type "Float (single-precision)"))
  (`parent.ReceiveTick` DeltaSeconds))

(event `InputAction|pick_up`
  (params (Key :type "Key Structure"))
  (bind _pickup_bp_dooritem (`self.PickUp_BP_DoorItem`))
  (bind (_relativelocation_x _relativelocation_y _relativelocation_z) (`KismetMathLibrary.BreakVector` (`SceneComponent.RelativeLocation` _pickup_bp_dooritem)))
  (bind (_relativelocation_x_2 _relativelocation_y_2 _relativelocation_z_2) (`KismetMathLibrary.BreakVector` (`SceneComponent.RelativeLocation` (`self.Sphere`))))
  (:`Pressed`
    (if (`self.Hovered`)
      (if (`self.Discovered`)
        (`/Engine/EditorBlueprintResources/StandardMacros.DoOnce` false
          (:`Completed`
            (set `self.was_clicked` true)
            (set `self.Active` false)
            (`GameplayStatics.PlaySoundAtLocation` "/Game/Audio/cabinet/drawer_sound_cue.drawer_sound_cue" (`SceneComponent.RelativeLocation` (`self.StaticMesh`)) (struct) 1.0 1.0 0.0 null null null)
            (bind (_direction _wysuniecie) (`Timeline|Timeline_0`)
              (:`Update`
                (`SceneComponent.K2_SetRelativeLocation` (`self.Sphere`) (`KismetMathLibrary.MakeVector` _relativelocation_x_2 _wysuniecie _relativelocation_z_2) false false)
                (`SceneComponent.K2_SetRelativeLocation` _pickup_bp_dooritem (`KismetMathLibrary.MakeVector` _relativelocation_x _wysuniecie _relativelocation_z) false false))
              (:`Finished`
                (bind _aspick_up_bp_door_item (cast `/Game/Blueprints/PickUp/PickUp_BP_DoorItem` (`ChildActorComponent.ChildActor` (`self.PickUp_BP_DoorItem`))))
                (`SphereComponent.SetSphereRadius` (`/Game/Blueprints/PickUp/PickUp_BP.Collision` _aspick_up_bp_door_item) 305.0 true)
                (`self.DisableInput` (`GameplayStatics.GetPlayerController` 0))
                (bind _foundwidgets (`WidgetBlueprintLibrary.GetAllWidgetsOfClass` "/Game/HUD/text_bot_screen.text_bot_screen_C"))
                (`/Game/HUD/text_bot_screen.ShowMessage` _foundwidgets "Got it!" 1.0)
                (set `self.completed` true)))))))))

(event `self.Collision.OnComponentBeginOverlap`
  (params (OverlappedComponent :type "PrimitiveComponent Object Reference") (OtherActor :type "Actor Object Reference") (OtherComp :type "PrimitiveComponent Object Reference") (OtherBodyIndex :type Integer) (bFromSweep :type Boolean) (SweepResult :type "HitResult Structure (by ref)"))
  (bind _returnvalue (`GameplayStatics.GetPlayerController` 0))
  (bind _asfirst_person_character (cast `/Game/FirstPersonBP/Blueprints/FirstPersonCharacter` (`GameplayStatics.GetPlayerCharacter` 0) :!pure true))
  (bind _returnvalue_2 (`GameplayStatics.GetActorOfClass` "/Game/Blueprints/PickUp/kitchen_cabinet.kitchen_cabinet_C"))
  (if (`/Game/Blueprints/PickUp/kitchen_cabinet.was_clicked` _returnvalue_2)
    (if (`self.was_clicked`)
      (set `self.Active` false)
      (if (== _asfirst_person_character (stale `self.Collision.OnComponentEndOverlap` OtherActor)) :!label _label
        (set `self.Can_interact` false)
        (`self.DisableInput` _returnvalue))
      (else
        (set `self.Active` true)
        (if (== OtherActor _asfirst_person_character)
          (set `self.Can_interact` true)
          (`self.EnableInput` _returnvalue))))
    (else
      (set `self.Active` false))))

(event `self.Collision.OnComponentEndOverlap`
  (params (OverlappedComponent :type "PrimitiveComponent Object Reference") (OtherActor :type "Actor Object Reference") (OtherComp :type "PrimitiveComponent Object Reference") (OtherBodyIndex :type Integer))
  (goto _label))

(fn `UserConstructionScript`
  (`parent.UserConstructionScript`))