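; Flare (raca) pickup that gives the first-person player a throwable.
; The collision overlap toggles interaction and input for the player, and the pick_up action also requires the item to be hovered.
; Pickup selects the flare as the throwable, increments the throw count, hides the mesh, and plays a sound at the Sphere's relative location.
; A Pickup_flare widget shows for a short delay before the actor destroys itself.
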(event `self.PickUp`)

(event `InputAction|pick_up`
  (params (Key :type "Key Structure"))
  (bind _returnvalue (`GameplayStatics.GetPlayerController` 0))
  (:`Pressed`
    (if (and (`self.Hovered`) (`self.Can_interact`))
      (bind _asfirst_person_character (cast `/Game/FirstPersonBP/Blueprints/FirstPersonCharacter` (`GameplayStatics.GetPlayerCharacter` 0)))
      (set `/Game/FirstPersonBP/Blueprints/FirstPersonCharacter.ChooseThrowable` 2 _asfirst_person_character)
      (set `/Game/FirstPersonBP/Blueprints/FirstPersonCharacter.is_destroyed_pickup_item` true _asfirst_person_character)
      (set `/Game/FirstPersonBP/Blueprints/FirstPersonCharacter.Throws` (+ (`/Game/FirstPersonBP/Blueprints/FirstPersonCharacter.Throws` _asfirst_person_character) 1) _asfirst_person_character)
      (bind _returnvalue_2 (`|CreateWidget` "/Game/HUD/pickup_flare.pickup_flare_C" _returnvalue))
      (`UserWidget.AddToViewport` _returnvalue_2 0)
      (`self.DisableInput` _returnvalue)
      (`SceneComponent.SetVisibility` (`self.Sphere`) false false)
      (`GameplayStatics.PlaySoundAtLocation` "/Game/Audio/Latarka/szuranie1_ciszej.szuranie1_ciszej" (`SceneComponent.RelativeLocation` (`self.Sphere`)) (struct) 1.0 1.0 0.0 null null null)
      (`KismetSystemLibrary.Delay` 2.0)
      (`Widget.RemoveFromParent` _returnvalue_2)
      (set `/Game/FirstPersonBP/Blueprints/FirstPersonCharacter.is_destroyed_pickup_item` true _asfirst_person_character)
      (`self.K2_DestroyActor`))))

(event `self.Collision.OnComponentBeginOverlap`
  (params (OverlappedComponent :type "PrimitiveComponent Object Reference") (OtherActor :type "Actor Object Reference") (OtherComp :type "PrimitiveComponent Object Reference") (OtherBodyIndex :type Integer) (bFromSweep :type Boolean) (SweepResult :type "HitResult Structure (by ref)"))
  (if (== OtherActor (`self.Player ref`))
    (set `self.Can_interact` true)
    (`self.EnableInput` (`GameplayStatics.GetPlayerController` 0))))

(event `self.Collision.OnComponentEndOverlap`
  (params (OverlappedComponent :type "PrimitiveComponent Object Reference") (OtherActor :type "Actor Object Reference") (OtherComp :type "PrimitiveComponent Object Reference") (OtherBodyIndex :type Integer))
  (if (== (`self.Player ref`) OtherActor)
    (set `self.Can_interact` false)
    (`self.DisableInput` (`GameplayStatics.GetPlayerController` 0))))

(fn `UserConstructionScript`
  (`parent.UserConstructionScript`))