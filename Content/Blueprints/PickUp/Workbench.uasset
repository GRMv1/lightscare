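; Workbench interactable that refills the player's Throws from 0 to 1 on the pick_up input, playing a sound and removing the craft prompt.
; Collision overlap sets CanInteract, which combines with Hovered to gate crafting.
; Tick enables the interaction sphere only when the player's Quest1 array reaches a set length, otherwise shrinking it to zero.
; Paired DoOnce nodes on Tick toggle the "press E to craft" widget and actor input as eligibility changes.
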(event `self.Collision.OnComponentBeginOverlap`
  (params (OverlappedComponent :type "PrimitiveComponent Object Reference") (OtherActor :type "Actor Object Reference") (OtherComp :type "PrimitiveComponent Object Reference") (OtherBodyIndex :type Integer) (bFromSweep :type Boolean) (SweepResult :type "HitResult Structure (by ref)"))
  (if (== OtherActor (`self.Player ref`))
    (set `self.Can_interact` true)))

(event `self.Collision.OnComponentEndOverlap`
  (params (OverlappedComponent :type "PrimitiveComponent Object Reference") (OtherActor :type "Actor Object Reference") (OtherComp :type "PrimitiveComponent Object Reference") (OtherBodyIndex :type Integer))
  (if (== (`self.Player ref`) OtherActor)
    (set `self.Can_interact` false)))

(event `InputAction|pick_up`
  (params (Key :type "Key Structure"))
  (:`Pressed`
    (`self.EnableInput` (`GameplayStatics.GetPlayerController` 0))
    (if (and (`self.Can_interact`) (`self.Hovered`))
      (if (== (`/Game/FirstPersonBP/Blueprints/FirstPersonCharacter.Throws` (`self.Player ref`)) 0)
        (set `/Game/FirstPersonBP/Blueprints/FirstPersonCharacter.Throws` 1 (`self.Player ref`))
        (`GameplayStatics.PlaySoundAtLocation` "/Game/Audio/Various/workbench.workbench" (`self.K2_GetActorLocation`) (struct) 1.0 1.0 0.0 null null null)
        (`Widget.RemoveFromParent` (stale `self.ReceiveTick` _returnvalue_2))))))

(event `self.ReceiveTick`
  (params (DeltaSeconds :type "Float (single-precision)"))
  (bind _returnvalue (`GameplayStatics.GetPlayerController` 0))
  (`parent.ReceiveTick` DeltaSeconds)
  (if (== (`KismetArrayLibrary.Array_LastIndex` (`/Game/FirstPersonBP/Blueprints/FirstPersonCharacter.Quest1` (`self.Player ref`))) 3)
    (`SphereComponent.SetSphereRadius` (`self.Collision`) 150.0 true)
    (if (and (`self.Can_interact`) (`self.Hovered`) (== (`/Game/FirstPersonBP/Blueprints/FirstPersonCharacter.Throws` (`self.Player ref`)) 0))
      (`/Engine/EditorBlueprintResources/StandardMacros.DoOnce` false :!label _label
        (:`Completed`
          (bind _returnvalue_2 (`|CreateWidget` "/Game/HUD/PressEToCraft.PressEToCraft_C" _returnvalue))
          (`UserWidget.AddToViewport` _returnvalue_2 0)
          (`self.EnableInput` _returnvalue)
          (goto _label_2 :!via `Reset`)))
      (else
        (`/Engine/EditorBlueprintResources/StandardMacros.DoOnce` true :!label _label_2
          (:`Completed`
            (`Widget.RemoveFromParent` _returnvalue_2)
            (`self.DisableInput` _returnvalue)
            (goto _label :!via `Reset`)))))
    (else
      (`SphereComponent.SetSphereRadius` (`self.Collision`) 0.0 true))))

(fn `UserConstructionScript`
  (`parent.UserConstructionScript`))