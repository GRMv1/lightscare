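; Locked door that opens and closes on the pick_up input when the player holds the matching key.
; Overlapping Collision shows a key-needed widget, removed if the character's DoorItems entry at DoorItemValue is true, which also enables input; leaving disables input.
; Pressing pick_up while Hovered rechecks the key and plays or reverses a timeline that yaws Sphere.
; Tick derives ClosedDoor from the timeline value and toggles the PressE prompt with Hovered.
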(event `InputAction|pick_up`
  (params (Key :type "Key Structure"))
  (:`Pressed`
    (bind _asfirst_person_character (cast `/Game/FirstPersonBP/Blueprints/FirstPersonCharacter` (`GameplayStatics.GetPlayerCharacter` 0)))
    (for (_array_element _array_index) (`/Game/FirstPersonBP/Blueprints/FirstPersonCharacter.door_items` _asfirst_person_character)
      (if (and _array_element (== _array_index (`self.door_item_value`)))
        (if (`self.Hovered`)
          (if true
            (if (`self.closed_door`)
              (bind (_direction _door_open) (`Timeline|Timeline_0` :!label _label)
                (:`Update`
                  (`SceneComponent.K2_SetRelativeRotation` (`self.Sphere`) (`KismetMathLibrary.MakeRotator` 0.0 0.0 _door_open) false false)))
              (else
                (goto _label :!via `Reverse`)))))))))

(event `self.ReceiveTick`
  (params (DeltaSeconds :type "Float (single-precision)"))
  (set `self.closed_door` (< (stale `InputAction|pick_up` _door_open) 1.0))
  (if (`self.Hovered`)
    (if (not (`self.is_widget`))
      (bind _returnvalue (`|CreateWidget` "/Game/HUD/PressE.PressE_C" (`GameplayStatics.GetPlayerController` 0)))
      (set `self.is_widget` true)
      (`UserWidget.AddToViewport` _returnvalue 0))
    (elif (`self.is_widget`)
      (`Widget.RemoveFromParent` _returnvalue)
      (set `self.is_widget` false))))

(event `self.Collision.OnComponentBeginOverlap`
  (params (OverlappedComponent :type "PrimitiveComponent Object Reference") (OtherActor :type "Actor Object Reference") (OtherComp :type "PrimitiveComponent Object Reference") (OtherBodyIndex :type Integer) (bFromSweep :type Boolean) (SweepResult :type "HitResult Structure (by ref)"))
  (if (== OtherActor (`self.Player ref`))
    (set `self.Can_interact` true)
    (bind _asfirst_person_character (cast `/Game/FirstPersonBP/Blueprints/FirstPersonCharacter` OtherActor))
    (bind _returnvalue (`|CreateWidget` "/Game/HUD/pressdoor_need.pressdoor_need_C" (`GameplayStatics.GetPlayerController` 0)))
    (`UserWidget.AddToViewport` _returnvalue 0)
    (for (_array_element _array_index) (`/Game/FirstPersonBP/Blueprints/FirstPersonCharacter.door_items` _asfirst_person_character)
      (if (and _array_element (== _array_index (`self.door_item_value`)))
        (`Widget.RemoveFromParent` _returnvalue)
        (`self.EnableInput` (`GameplayStatics.GetPlayerController` 0))
        (set `self.enable_input` true)))))

(event `self.Collision.OnComponentEndOverlap`
  (params (OverlappedComponent :type "PrimitiveComponent Object Reference") (OtherActor :type "Actor Object Reference") (OtherComp :type "PrimitiveComponent Object Reference") (OtherBodyIndex :type Integer))
  (if (== (`self.Player ref`) OtherActor)
    (set `self.Can_interact` false)
    (cast `/Game/FirstPersonBP/Blueprints/FirstPersonCharacter` OtherActor)
    (if (not (`self.enable_input`))
      (`Widget.RemoveFromParent` (stale `self.Collision.OnComponentBeginOverlap` _returnvalue)))
    (`self.DisableInput` (`GameplayStatics.GetPlayerController` 0))))

(fn `UserConstructionScript`
  (`parent.UserConstructionScript`))