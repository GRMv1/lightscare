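; Key-locked swinging door (shed gate) that the first-person player opens and closes with the use action.
; A box overlap enables input for the player, and use only responds once Discovered, reset at BeginPlay, is set true.
; It unlocks if the player's DoorItems flag at DoorItemValue is set, otherwise playing a sound and showing a locked message.
; When unlocked, a timeline rotates the Sphere component's yaw, reversing to close.
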(event `self.ReceiveBeginPlay`
  (`parent.ReceiveBeginPlay`)
  (set `self.Discovered` false))

(event `self.Box.OnComponentBeginOverlap`
  (params (OverlappedComponent :type "PrimitiveComponent Object Reference") (OtherActor :type "Actor Object Reference") (OtherComp :type "PrimitiveComponent Object Reference") (OtherBodyIndex :type Integer) (bFromSweep :type Boolean) (SweepResult :type "HitResult Structure (by ref)"))
  (if (== OtherActor (cast `/Game/FirstPersonBP/Blueprints/FirstPersonCharacter` (`GameplayStatics.GetPlayerCharacter` 0) :!pure true))
    (`self.EnableInput` (`GameplayStatics.GetPlayerController` 0))
    (set `self.Can_interact` true)))

(event `self.Box.OnComponentEndOverlap`
  (params (OverlappedComponent :type "PrimitiveComponent Object Reference") (OtherActor :type "Actor Object Reference") (OtherComp :type "PrimitiveComponent Object Reference") (OtherBodyIndex :type Integer))
  (if (== (cast `/Game/FirstPersonBP/Blueprints/FirstPersonCharacter` (`GameplayStatics.GetPlayerCharacter` 0) :!pure true) OtherActor)
    (`self.DisableInput` (`GameplayStatics.GetPlayerController` 0))
    (set `self.Can_interact` false)))

(event `InputAction|use`
  (params (Key :type "Key Structure"))
  (bind _open_door (`self.open_door`))
  (bind _try_open_door (`self.try_open_door`))
  (:`Pressed`
    (if (`self.Discovered`)
      (for (_array_element _array_index) (`/Game/FirstPersonBP/Blueprints/FirstPersonCharacter.door_items` (cast `/Game/FirstPersonBP/Blueprints/FirstPersonCharacter` (`GameplayStatics.GetPlayerCharacter` 0) :!pure true))
        (if (and _array_element (== _array_index (`self.door_item_value`)))
          (set `self.locked_door` false)))
      (if (`self.locked_door`)
        (`AudioComponent.Stop` _try_open_door)
        (`AudioComponent.Play` _try_open_door 0.0)
        (bind _foundwidgets (`WidgetBlueprintLibrary.GetAllWidgetsOfClass` "/Game/HUD/text_bot_screen.text_bot_screen_C"))
        (`/Game/HUD/text_bot_screen.ShowMessage` :`self` _foundwidgets :`text` "Door locked " :`time` 3.0)
        (else
          (`AudioComponent.Stop` _open_door)
          (`AudioComponent.Play` _open_door 0.0)
          (if (`self.closed_door`)
            (bind (_direction _door_open) (`Timeline|Timeline_0` :!label _label)
              (:`Update`
                (`SceneComponent.K2_SetRelativeRotation` (`self.Sphere`) (`KismetMathLibrary.MakeRotator` 0.0 0.0 _door_open) false false)
                (set `self.closed_door` (< _door_open 1.0))))
            (else
              (goto _label :!via `Reverse`))))))))

(fn `UserConstructionScript`
  (`parent.UserConstructionScript`))