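; Fuse pickup ("bezpiecznik") that the player collects with the pick_up input once it is both hovered and discovered.
; Its collision overlap toggles input and CanInteract for the player, and Discovered resets on BeginPlay.
; Collecting plays a sound, flags the FirstPersonCharacter, adds "fuse" to the inventory and destroys the actor.
; It also calls SetFuseTrue on every Mob_Ai in the level, with no active distance filter.
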(event `self.ReceiveBeginPlay`
  (`parent.ReceiveBeginPlay`)
  (set `self.Discovered` false))

(event `InputAction|pick_up`
  (params (Key :type "Key Structure"))
  (:`Pressed`
    (if (`self.Hovered`)
      (if (`self.Discovered`)
        (`AudioComponent.Play` (`self.pickupSound`) 0.0)
        (bind _asfirst_person_character (cast `/Game/FirstPersonBP/Blueprints/FirstPersonCharacter` (`GameplayStatics.GetPlayerCharacter` 0)))
        (set `/Game/FirstPersonBP/Blueprints/FirstPersonCharacter.has_bezpiecznik` true _asfirst_person_character)
        (`/Game/FirstPersonBP/Blueprints/FirstPersonCharacter.addInventoryItem` _asfirst_person_character "fuse")
        (`self.K2_DestroyActor`)
        (set `/Game/FirstPersonBP/Blueprints/FirstPersonCharacter.is_destroyed_pickup_item` true _asfirst_person_character)
        (`self.K2_DestroyActor`)
        (bind _outactors (`GameplayStatics.GetAllActorsOfClass` "/Game/ThirdPersonBP/AI/Mob_Ai.Mob_Ai_C"))
        (for _array_element _outactors
          (`/Game/ThirdPersonBP/AI/Mob_Ai.SetFuseTrue` _array_element)
          (set `/Game/FirstPersonBP/Blueprints/FirstPersonCharacter.distanceFromThrowitem` 1230000.0 _asfirst_person_character))))))

(event `self.Collision.OnComponentBeginOverlap`
  (params (OverlappedComponent :type "PrimitiveComponent Object Reference") (OtherActor :type "Actor Object Reference") (OtherComp :type "PrimitiveComponent Object Reference") (OtherBodyIndex :type Integer) (bFromSweep :type Boolean) (SweepResult :type "HitResult Structure (by ref)"))
  (if (== OtherActor (cast `/Game/FirstPersonBP/Blueprints/FirstPersonCharacter` (`GameplayStatics.GetPlayerCharacter` 0) :!pure true))
    (set `self.Can_interact` true)
    (`self.EnableInput` (`GameplayStatics.GetPlayerController` 0))))

(event `self.Collision.OnComponentEndOverlap`
  (params (OverlappedComponent :type "PrimitiveComponent Object Reference") (OtherActor :type "Actor Object Reference") (OtherComp :type "PrimitiveComponent Object Reference") (OtherBodyIndex :type Integer))
  (if (== (cast `/Game/FirstPersonBP/Blueprints/FirstPersonCharacter` (`GameplayStatics.GetPlayerCharacter` 0) :!pure true) OtherActor)
    (set `self.Can_interact` false)
    (`self.DisableInput` (`GameplayStatics.GetPlayerController` 0))))

(fn `UserConstructionScript`
  (`parent.UserConstructionScript`))