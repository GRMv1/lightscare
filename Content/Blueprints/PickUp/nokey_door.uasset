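; Door actor that opens without a key when the player presses the pick_up input.
; A Box overlap enables input and CanInteract for the first-person player until they leave, unless the door was already used.
; The press requires Hovered and Discovered, neither set in these graphs, then plays OpenDoor and an Openclose timeline that yaws the Sphere component.
; When the timeline finishes, WasUsed locks the door and Active clears.
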(event `self.Box.OnComponentBeginOverlap`
  (params (OverlappedComponent :type "PrimitiveComponent Object Reference") (OtherActor :type "Actor Object Reference") (OtherComp :type "PrimitiveComponent Object Reference") (OtherBodyIndex :type Integer) (bFromSweep :type Boolean) (SweepResult :type "HitResult Structure (by ref)"))
  (if (== OtherActor (cast `/Game/FirstPersonBP/Blueprints/FirstPersonCharacter` (`GameplayStatics.GetPlayerCharacter` 0) :!pure true))
    (if (`self.was_used`)
      (set `self.Active` false)
      (else
        (set `self.Can_interact` true)
        (`self.EnableInput` (`GameplayStatics.GetPlayerController` 0))))))

(event `self.Box.OnComponentEndOverlap`
  (params (OverlappedComponent :type "PrimitiveComponent Object Reference") (OtherActor :type "Actor Object Reference") (OtherComp :type "PrimitiveComponent Object Reference") (OtherBodyIndex :type Integer))
  (if (== (cast `/Game/FirstPersonBP/Blueprints/FirstPersonCharacter` (`GameplayStatics.GetPlayerCharacter` 0) :!pure true) OtherActor)
    (set `self.Can_interact` false)
    (`self.DisableInput` (`GameplayStatics.GetPlayerController` 0))))

(event `InputAction|pick_up`
  (params (Key :type "Key Structure"))
  (bind _open_door (`self.open door`))
  (bind (_relativerotation_roll _relativerotation_pitch) (`KismetMathLibrary.BreakRotator` (`SceneComponent.RelativeRotation` (`self.Sphere`))))
  (:`Pressed`
    (if (`self.Hovered`)
      (if (`self.Discovered`)
        (if (not (`self.was_used`))
          (`AudioComponent.Play` _open_door 0.0)
          (bind (_direction _open_close) (`Timeline|open/close`)
            (:`Update`
              (`SceneComponent.K2_SetRelativeLocationAndRotation` (`self.Sphere`) (0.0 0.0 0.0) (`KismetMathLibrary.MakeRotator` _relativerotation_roll _relativerotation_pitch _open_close) false false))
            (:`Finished`
              (set `self.was_used` true)
              (`AudioComponent.Stop` _open_door)
              (set `self.Active` false))))))))

(fn `UserConstructionScript`
  (`parent.UserConstructionScript`))