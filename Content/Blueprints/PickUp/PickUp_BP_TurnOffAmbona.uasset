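; Interactable switch that toggles every Light_ambona actor in the level when the player presses pick_up.
; A collision volume sets CanInteract and enables input only while the player overlaps it.
; The press requires Hovered, CanInteract and Discovered, then plays the Car_lights sound at the Sphere's relative location and calls TurnOnOffAmbonaLight on each light.
; Discovered resets to false on BeginPlay and is never set true in this graph.
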(event `self.ReceiveBeginPlay`
  (`parent.ReceiveBeginPlay`)
  (set `self.Discovered` false))

(event `self.PickUp`)

(event `InputAction|pick_up`
  (params (Key :type "Key Structure"))
  (:`Pressed`
    (if (and (`self.Hovered`) (`self.Can_interact`))
      (if (`self.Discovered`)
        (cast `/Game/FirstPersonBP/Blueprints/FirstPersonCharacter` (`GameplayStatics.GetPlayerCharacter` 0))
        (`GameplayStatics.PlaySoundAtLocation` "/Game/Audio/przelacznik/car_lights.car_lights" (`SceneComponent.RelativeLocation` (`self.Sphere`)) (struct) 1.0 1.0 0.0 null null null)
        (bind _outactors (`GameplayStatics.GetAllActorsOfClass` "/Game/Blueprints/light/light_ambona.light_ambona_C"))
        (for _array_element _outactors
          (`/Game/Blueprints/light/light_ambona.TurnOnOffAmbonaLight` _array_element))))))

(event `self.Collision.OnComponentBeginOverlap`
  (params (OverlappedComponent :type "PrimitiveComponent Object Reference") (OtherActor :type "Actor Object Reference") (OtherComp :type "PrimitiveComponent Object Reference") (OtherBodyIndex :type Integer) (bFromSweep :type Boolean) (SweepResult :type "HitResult Structure (by ref)"))
  (if (== OtherActor (cast `/Game/FirstPersonBP/Blueprints/FirstPersonCharacter` (`GameplayStatics.GetPlayerCharacter` 0) :!pure true))
    (set `self.Can_interact` true)
    (`self.EnableInput` (`GameplayStatics.GetPlayerController` 0))))

(event `self.Collision.OnComponentEndOverlap`
  (params (OverlappedComponent :type "PrimitiveComponent Object Reference") (OtherActor :type "Actor Object Reference") (OtherComp :type "PrimitiveComponent Object Reference") (OtherBodyIndex :type Integer))
  (if (== (cast `/Game/FirstPersonBP/Blueprints/FirstPersonCharacter` (`GameplayStatics.GetPlayerCharacter` 0) :!pure true) OtherActor)
    (set `self.Can_interact` false)
    (`self.DisableInput` (`GameplayStatics.GetPlayerController` 0))))

(fn `UserConstructionScript`
  (`parent.UserConstructionScript`))