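; Battery pickup that adds a battery to the first-person character's inventory.
; A collision component toggles interaction and input as the player enters or leaves it.
; Pressing pick_up while it is hovered and discovered plays a sound and records whether the battery is full in the character's TableBattery array.
; It then disappears rather than being destroyed, and the character keeps a reference to it in Batteries.
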(event `self.ReceiveBeginPlay`
  (`parent.ReceiveBeginPlay`))

(event `InputAction|pick_up`
  (params (Key :type "Key Structure"))
  (:`Pressed`
    (if (`self.Hovered`)
      (if (`self.Discovered`)
        (`GameplayStatics.PlaySound2D` "/Game/Audio/Latarka/szuranie1_ciszej.szuranie1_ciszej" 1.0 1.0 0.0 null null)
        (bind _asfirst_person_character (cast `/Game/FirstPersonBP/Blueprints/FirstPersonCharacter` (`GameplayStatics.GetPlayerCharacter` 0)))
        (`/Game/FirstPersonBP/Blueprints/FirstPersonCharacter.addInventoryItem` _asfirst_person_character "battery")
        (if (`self.IsBatteryFull`)
          (bind _tablebattery (`/Game/FirstPersonBP/Blueprints/FirstPersonCharacter.TableBattery` _asfirst_person_character))
          (`KismetArrayLibrary.Array_Add` _tablebattery true)
          (else
            (`KismetArrayLibrary.Array_Add` _tablebattery)))
        (set `/Game/FirstPersonBP/Blueprints/FirstPersonCharacter.is_destroyed_pickup_item` true _asfirst_person_character)
        (`self.Set Actor Disappeared` true)
        (`KismetArrayLibrary.Array_Add` (`/Game/FirstPersonBP/Blueprints/FirstPersonCharacter.batteries` (cast `/Game/FirstPersonBP/Blueprints/FirstPersonCharacter` (`GameplayStatics.GetPlayerCharacter` 0) :!pure true)) self)))))

(event `self.Collision.OnComponentBeginOverlap`
  (params (OverlappedComponent :type "PrimitiveComponent Object Reference") (OtherActor :type "Actor Object Reference") (OtherComp :type "PrimitiveComponent Object Reference") (OtherBodyIndex :type Integer) (bFromSweep :type Boolean) (SweepResult :type "HitResult Structure (by ref)"))
  (if (== OtherActor (cast `/Game/FirstPersonBP/Blueprints/FirstPersonCharacter` (`GameplayStatics.GetPlayerCharacter` 0) :!pure true))
    (set `self.Can_interact` true)
    (`self.EnableInput` (`GameplayStatics.GetPlayerController` 0))))

(event `self.Collision.OnComponentEndOverlap`
  (params (OverlappedComponent :type "PrimitiveComponent Object Reference") (OtherActor :type "Actor Object Reference") (OtherComp :type "PrimitiveComponent Object Reference") (OtherBodyIndex :type Integer))
  (if (== (cast `/Game/FirstPersonBP/Blueprints/FirstPersonCharacter` (`GameplayStatics.GetPlayerCharacter` 0) :!pure true) OtherActor)
    (set `self.Can_interact` false)
    (`self.DisableInput` (`GameplayStatics.GetPlayerController` 0))))

(fn `UserConstructionScript`
  (`parent.UserConstructionScript`))