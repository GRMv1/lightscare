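; Interactable kitchen cabinet pickup whose drawer slides out once, gated behind the Coat actor having been clicked.
; Collision overlap checks the Coat and its own WasClicked state, then sets Active and enables input for the player, disabling it on exit.
; The pick_up action, if Discovered (reset at BeginPlay, not set true here), plays a drawer sound and a timeline moving Sphere along Y, then disables input.
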(event `self.ReceiveBeginPlay`
  (`parent.ReceiveBeginPlay`)
  (set `self.Discovered` false))

(event `InputAction|pick_up`
  (params (Key :type "Key Structure"))
  (bind (_relativelocation_x _relativelocation_y _relativelocation_z) (`KismetMathLibrary.BreakVector` (`SceneComponent.RelativeLocation` (`self.Sphere`))))
  (:`Pressed`
    (if (`self.Discovered`)
      (`/Engine/EditorBlueprintResources/StandardMacros.DoOnce` false
        (:`Completed`
          (set `self.was_clicked` true)
          (set `self.Active` false)
          (`GameplayStatics.PlaySoundAtLocation` "/Game/Audio/cabinet/drawer_sound_cue.drawer_sound_cue" (`SceneComponent.RelativeLocation` (`self.szafka`)) (struct) 1.0 1.0 0.0 null null null)
          (bind (_direction _wysuniecie) (`Timeline|wysuniecie`)
            (:`Update`
              (`SceneComponent.K2_SetRelativeLocation` (`self.Sphere`) (`KismetMathLibrary.MakeVector` _relativelocation_x _wysuniecie _relativelocation_z) false false))
            (:`Finished`
              (`self.DisableInput` (`GameplayStatics.GetPlayerController` 0)))))))))

(event `self.Collision.OnComponentBeginOverlap`
  (params (OverlappedComponent :type "PrimitiveComponent Object Reference") (OtherActor :type "Actor Object Reference") (OtherComp :type "PrimitiveComponent Object Reference") (OtherBodyIndex :type Integer) (bFromSweep :type Boolean) (SweepResult :type "HitResult Structure (by ref)"))
  (bind _returnvalue (`GameplayStatics.GetPlayerController` 0))
  (bind _returnvalue_2 (`GameplayStatics.GetActorOfClass` "/Game/Blueprints/PickUp/coat.coat_C"))
  (if (`/Game/Blueprints/PickUp/coat.was_clicked` _returnvalue_2)
    (if (`self.was_clicked`)
      (set `self.Active` false :!label _label)
      (`self.DisableInput` _returnvalue :!label _label_2)
      (else
        (set `self.Active` true)
        (if (== OtherActor (`self.Player ref`))
          (set `self.Can_interact` true)
          (`self.EnableInput` _returnvalue))))
    (else
      (goto _label))))

(event `self.Collision.OnComponentEndOverlap`
  (params (OverlappedComponent :type "PrimitiveComponent Object Reference") (OtherActor :type "Actor Object Reference") (OtherComp :type "PrimitiveComponent Object Reference") (OtherBodyIndex :type Integer))
  (if (== (`self.Player ref`) OtherActor)
    (set `self.Can_interact` false)
    (goto _label_2)))

(fn `UserConstructionScript`
  (`parent.UserConstructionScript`))