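; PickUp_BP is a pickup actor that the first-person player discovers by hovering it with their light on.
; Tick sets Discovered, then toggles custom depth and stencil on Sphere and its child primitives to mark it while hovered, active and discovered.
; Hovered is not set in this graph.
; The PickUp and overlap events are empty, and the logic toggling interaction and input is disconnected.
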(event `self.ReceiveBeginPlay`
  (bind _asfirst_person_character (cast `/Game/FirstPersonBP/Blueprints/FirstPersonCharacter` (`GameplayStatics.GetPlayerCharacter` 0)))
  (set `self.Player ref` _asfirst_person_character))

(event `self.ReceiveTick`
  (params (DeltaSeconds :type "Float (single-precision)"))
  (bind _sphere (`self.Sphere`))
  (bind _children (`SceneComponent.GetChildrenComponents` _sphere false))
  (if (and (`self.Hovered`) (not (`self.Discovered`)))
    (if (`/Game/FirstPersonBP/Blueprints/FirstPersonCharacter.is_light_on` (`self.Player ref`))
      (set `self.Discovered` true))
    (elif (and (`self.Hovered`) (`self.Active`) (`self.Discovered`))
      (`PrimitiveComponent.SetRenderCustomDepth` _sphere true)
      (`PrimitiveComponent.SetCustomDepthStencilValue` _sphere 2)
      (for _array_element _children
        (bind _asprimitive_component (cast `PrimitiveComponent` _array_element))
        (`PrimitiveComponent.SetRenderCustomDepth` _asprimitive_component true)
        (`PrimitiveComponent.SetCustomDepthStencilValue` _asprimitive_component 2))
      (else
        (`PrimitiveComponent.SetRenderCustomDepth` _sphere false)
        (`PrimitiveComponent.SetCustomDepthStencilValue` _sphere 0)
        (for _array_element_2 _children
          (bind _asprimitive_component_2 (cast `PrimitiveComponent` _array_element_2))
          (`PrimitiveComponent.SetRenderCustomDepth` _asprimitive_component_2 false)
          (`PrimitiveComponent.SetCustomDepthStencilValue` _asprimitive_component_2 0))))))

(event `self.Collision.OnComponentBeginOverlap`
  (params (OverlappedComponent :type "PrimitiveComponent Object Reference") (OtherActor :type "Actor Object Reference") (OtherComp :type "PrimitiveComponent Object Reference") (OtherBodyIndex :type Integer) (bFromSweep :type Boolean) (SweepResult :type "HitResult Structure (by ref)")))

(event `self.Collision.OnComponentEndOverlap`
  (params (OverlappedComponent :type "PrimitiveComponent Object Reference") (OtherActor :type "Actor Object Reference") (OtherComp :type "PrimitiveComponent Object Reference") (OtherBodyIndex :type Integer)))

(event `PickUp`)

(fn `UserConstructionScript`)