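; Wall or world switch actor that, on the use input, stuns nearby Mob_Ai enemies and sounds an alarm.
; Overlapping the player enables input; a hover flag toggles the PressE prompt on Tick.
; Stun lights and the handle timeline start only when a mob is within range.
; The timeline value also gates reuse and, in a narrow window, shuts off lights and alarm.
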(event `self.Collision.OnComponentBeginOverlap`
  (params (OverlappedComponent :type "PrimitiveComponent Object Reference") (OtherActor :type "Actor Object Reference") (OtherComp :type "PrimitiveComponent Object Reference") (OtherBodyIndex :type Integer) (bFromSweep :type Boolean) (SweepResult :type "HitResult Structure (by ref)"))
  (if (== OtherActor (`self.Player ref`))
    (set `self.Can_interact` true)
    (`self.EnableInput` (`GameplayStatics.GetPlayerController` 0))))

(event `self.Collision.OnComponentEndOverlap`
  (params (OverlappedComponent :type "PrimitiveComponent Object Reference") (OtherActor :type "Actor Object Reference") (OtherComp :type "PrimitiveComponent Object Reference") (OtherBodyIndex :type Integer))
  (if (== (`self.Player ref`) OtherActor)
    (set `self.Can_interact` false)
    (`self.DisableInput` (`GameplayStatics.GetPlayerController` 0))))

(event `InputAction|use`
  (params (Key :type "Key Structure"))
  (bind (_relativelocation_x _relativelocation_y) (`KismetMathLibrary.BreakVector` (`SceneComponent.RelativeLocation` (`self.switch_handle`))))
  (:`Pressed`
    (if (`self.can_switch`)
      (set `self.is_on` true)
      (`GameplayStatics.PlaySoundAtLocation` "/Game/Audio/przelacznik/stun_switch.stun_switch" (`SceneComponent.RelativeLocation` (`self.Sphere`)) (struct) 1.0 1.0 0.0 null null null)
      (bind _returnvalue (`GameplayStatics.SpawnSound2D` "/Game/Audio/alarm/alarm.alarm" 1.0 1.0 0.0 null false false))
      (bind _outactors (`GameplayStatics.GetAllActorsOfClass` "/Game/ThirdPersonBP/AI/Mob_Ai.Mob_Ai_C"))
      (for _array_element _outactors
        (if (< (`KismetMathLibrary.Vector_Distance` (`self.K2_GetActorLocation` _array_element) (`self.K2_GetActorLocation`)) 7000.0)
          (`/Game/ThirdPersonBP/AI/Mob_Ai.stun` _array_element)
          (bind _outactors_2 (`GameplayStatics.GetAllActorsOfClass` "/Game/Blueprints/przelacznik/stun_light.stun_light_C"))
          (for _array_element_2 _outactors_2
            (`/Game/Blueprints/przelacznik/stun_light.StunLight` _array_element_2)
            (bind (_direction _switched) (`Timeline|Timeline_0` :!via `PlayFromStart`)
              (:`Update`
                (`SceneComponent.K2_SetRelativeLocation` (`self.switch_handle`) (`KismetMathLibrary.MakeVector` _relativelocation_x _relativelocation_y _switched) false false)
                (if (and (< _switched 20.0) (> _switched 16.0))
                  (for _array_element_3 _outactors_2
                    (`/Game/Blueprints/przelacznik/stun_light.StunLightOff` _array_element_3)
                    (`ActorComponent.SetActive` _returnvalue false false)))))))))))

(event `self.ReceiveTick`
  (params (DeltaSeconds :type "Float (single-precision)"))
  (set `self.can_switch` (not (and (< (stale `InputAction|use` _switched) 125.0) (> (stale `InputAction|use` _switched) 16.0))))
  (if (`self.Hovered`)
    (if (not (`self.is_widget`))
      (bind _returnvalue (`|CreateWidget` "/Game/HUD/PressE.PressE_C" (`GameplayStatics.GetPlayerController` 0)))
      (set `self.is_widget` true)
      (`UserWidget.AddToViewport` _returnvalue 0))
    (elif (`self.is_widget`)
      (`Widget.RemoveFromParent` _returnvalue)
      (set `self.is_widget` false))))

(fn `UserConstructionScript`
  (`parent.UserConstructionScript`))