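; Light switch Blueprint that toggles a set of lights and plays on/off click sounds.
; The ToggleLights event loops over the Lights array and toggles each light component's visibility.
; A FlipFlop inside the loop alternates the on and off cues at the Cube mesh's location, so it advances once per light rather than once per switch use.
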(event `Toggle Lights`
  (for _array_element (`self.Lights`)
    (`SceneComponent.ToggleVisibility` (`Light.LightComponent` _array_element) false)
    (`/Engine/EditorBlueprintResources/StandardMacros.FlipFlop`
      (:`A`
        (`GameplayStatics.PlaySoundAtLocation` "/Game/Audio/Latarka/On_Cue.On_Cue" (`SceneComponent.K2_GetComponentLocation` (`self.Cube`)) (struct) 1.0 1.0 0.0 null null null))
      (:`B`
        (`GameplayStatics.PlaySoundAtLocation` "/Game/Audio/Latarka/Off_Cue.Off_Cue" (`SceneComponent.K2_GetComponentLocation` (`self.Cube`)) (struct) 1.0 1.0 0.0 null null null)))))

(fn `UserConstructionScript`)