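; Trigger volume that shows a text hint after the player has spent some time inside it.
; Overlap events flag the player's presence, and a Delay on Tick counts roughly seconds, printing the counter for debug, up to a short first threshold, then a long one.
; At the threshold it sends TextToShow to the Text_bot_screen widget.
; Inventory-checking events update the neighbours' house hint; the Szopa one has no effect yet.
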(event `UpdateTextForNeighborsHouse`
  (bind _isitemonlist (`/Game/FirstPersonBP/Blueprints/FirstPersonCharacter.checkIsItemOnList` (cast `/Game/FirstPersonBP/Blueprints/FirstPersonCharacter` (`GameplayStatics.GetPlayerCharacter` 0) :!pure true) "neighborsNote"))
  (if (not _isitemonlist)
    (set `self.textToShow` "Maybe there is some note with code to open the doors.")))

(event `self.ReceiveActorBeginOverlap`
  (params (OtherActor :type "Actor Object Reference"))
  (cast `/Game/FirstPersonBP/Blueprints/FirstPersonCharacter` OtherActor)
  (set `self.isPlayerOverlap` true))

(event `UpdateTextForSzopa`
  (bind _asfirst_person_character (cast `/Game/FirstPersonBP/Blueprints/FirstPersonCharacter` (`GameplayStatics.GetPlayerCharacter` 0) :!pure true))
  (bind _isitemonlist (`/Game/FirstPersonBP/Blueprints/FirstPersonCharacter.checkIsItemOnList` _asfirst_person_character "wood"))
  (bind _isitemonlist_2 (`/Game/FirstPersonBP/Blueprints/FirstPersonCharacter.checkIsItemOnList` _asfirst_person_character "zippo"))
  (bind _isitemonlist_3 (`/Game/FirstPersonBP/Blueprints/FirstPersonCharacter.checkIsItemOnList` _asfirst_person_character "cloth"))
  (if (and _isitemonlist _isitemonlist_2 _isitemonlist_3)
    _))

(event `self.ReceiveActorEndOverlap`
  (params (OtherActor :type "Actor Object Reference"))
  (cast `/Game/FirstPersonBP/Blueprints/FirstPersonCharacter` OtherActor)
  (set `self.isPlayerOverlap` false))

(event `self.ReceiveTick`
  (params (DeltaSeconds :type "Float (single-precision)"))
  (`KismetSystemLibrary.Delay` 1.0)
  (if (`self.useShortTime`)
    (set `self.time` (`self.shortTime`))
    (else
      (set `self.time` (`self.longTime`))))
  (if (`self.isPlayerOverlap`)
    (`KismetSystemLibrary.PrintString` (`KismetStringLibrary.Conv_IntToString` (`self.counter`)))
    (if (< (`self.counter`) (`self.time`))
      (set `self.counter` (+ (`self.counter`) 1))
      (else
        (set `self.counter` 0)
        (set `self.useShortTime` false)
        (bind _foundwidgets (`WidgetBlueprintLibrary.GetAllWidgetsOfClass` "/Game/HUD/text_bot_screen.text_bot_screen_C"))
        (`/Game/HUD/text_bot_screen.ShowMessage` _foundwidgets (`self.textToShow`) 5.0)))))

(fn `UserConstructionScript`)