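; TriggerFuzeCounter is a trigger actor that starts a countdown when a Mob overlaps it, then clears the fuse on AI mobs.
; Tick records the start time on its first active frame and compares real-time seconds against the Time delay.
; On expiry it calls SetFuseFalse on every Mob_Ai, stopping the counter and destroying itself inside that loop.
; An item-list check for "torchThrow" is left unconnected.
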(event `self.ReceiveActorBeginOverlap`
  (params (OtherActor :type "Actor Object Reference"))
  (cast `/Game/ThirdPersonBP/AI/Mob` OtherActor)
  (set `self.isCounterActive` true))

(event `self.ReceiveTick`
  (params (DeltaSeconds :type "Float (single-precision)"))
  (if (`self.isCounterActive`)
    (if (> (`self.startTime`) 0.0)
      (if (> (- (`GameplayStatics.GetRealTimeSeconds`) (`self.startTime`)) (`self.time`))
        (bind _outactors (`GameplayStatics.GetAllActorsOfClass` "/Game/ThirdPersonBP/AI/Mob_Ai.Mob_Ai_C"))
        (for _array_element _outactors
          (`/Game/ThirdPersonBP/AI/Mob_Ai.SetFuseFalse` _array_element)
          (set `self.isCounterActive` false)
          (`self.K2_DestroyActor`)))
      (else
        (set `self.startTime` (`GameplayStatics.GetRealTimeSeconds`))))))

(fn `UserConstructionScript`)