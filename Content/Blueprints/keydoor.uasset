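; Key-locked door actor that a first-person character opens and closes with the use input.
; Entering its box shows prompt widgets and checks the character's DoorItems flag at DoorItemValue; a match removes the key-needed prompt and enables input.
; Use plays or reverses a rotation timeline, choosing direction from a closed state updated each Tick.
; Also contains a Hold macro distinguishing tap from hold, not used in the event graph.
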(event `self.door.OnBeginCursorOver`
  (params (TouchedComponent :type "PrimitiveComponent Object Reference")))

(event `self.door.OnEndCursorOver`
  (params (TouchedComponent :type "PrimitiveComponent Object Reference")))

(event `self.Box.OnComponentBeginOverlap`
  (params (OverlappedComponent :type "PrimitiveComponent Object Reference") (OtherActor :type "Actor Object Reference") (OtherComp :type "PrimitiveComponent Object Reference") (OtherBodyIndex :type Integer) (bFromSweep :type Boolean) (SweepResult :type "HitResult Structure (by ref)"))
  (bind _returnvalue (`GameplayStatics.GetPlayerController` 0))
  (set `self.inbox` "Visible")
  (bind _asfirst_person_character (cast `/Game/FirstPersonBP/Blueprints/FirstPersonCharacter` OtherActor))
  (bind _returnvalue_2 (`|CreateWidget` "/Game/HUD/PressE.PressE_C" _returnvalue))
  (`UserWidget.AddToViewport` _returnvalue_2 0)
  (bind _returnvalue_3 (`|CreateWidget` "/Game/HUD/pressdoor_need.pressdoor_need_C" _returnvalue))
  (`UserWidget.AddToViewport` _returnvalue_3 0)
  (for (_array_element _array_index) (`/Game/FirstPersonBP/Blueprints/FirstPersonCharacter.door_items` _asfirst_person_character)
    (if (and _array_element (== _array_index (`self.door_item_value`)))
      (`Widget.RemoveFromParent` _returnvalue_3)
      (`self.EnableInput` _returnvalue)
      (set `self.enable_input` true))))

(event `self.Box.OnComponentEndOverlap`
  (params (OverlappedComponent :type "PrimitiveComponent Object Reference") (OtherActor :type "Actor Object Reference") (OtherComp :type "PrimitiveComponent Object Reference") (OtherBodyIndex :type Integer))
  (set `self.inbox` "Hidden")
  (cast `/Game/FirstPersonBP/Blueprints/FirstPersonCharacter` OtherActor)
  (`Widget.RemoveFromParent` (stale `self.Box.OnComponentBeginOverlap` _returnvalue_2))
  (if (not (`self.enable_input`))
    (`Widget.RemoveFromParent` (stale `self.Box.OnComponentBeginOverlap` _returnvalue_3)))
  (`self.DisableInput` (`GameplayStatics.GetPlayerController` 0)))

(event `InputAction|use`
  (params (Key :type "Key Structure"))
  (:`Pressed`
    (if (`self.closed_door`)
      (bind (_direction _door_open) (`Timeline|door rotation` :!label _label)
        (:`Update`
          (`SceneComponent.K2_SetRelativeRotation` (`self.door`) (`KismetMathLibrary.MakeRotator` 0.0 0.0 _door_open) false false)))
      (else
        (goto _label :!via `Reverse`)))))

(event `self.ReceiveTick`
  (params (DeltaSeconds :type "Float (single-precision)"))
  (set `self.closed_door` (< (stale `InputAction|use` _door_open) 1.0)))

(fn `UserConstructionScript`)