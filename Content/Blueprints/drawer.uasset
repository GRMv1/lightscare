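; Interactive drawer that the player slides open and closed with the use input.
; A trigger box enables input while the FirstPersonCharacter overlaps it and disables it on exit.
; The use press toggles on IsOpen, calling open or close events whose separate timelines lerp the drawer mesh's relative location between closed and pulled-out positions.
; Each timeline updates IsOpen only when it finishes.
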(event `self.Box.OnComponentBeginOverlap`
  (params (OverlappedComponent :type "PrimitiveComponent Object Reference") (OtherActor :type "Actor Object Reference") (OtherComp :type "PrimitiveComponent Object Reference") (OtherBodyIndex :type Integer) (bFromSweep :type Boolean) (SweepResult :type "HitResult Structure (by ref)"))
  (cast `/Game/FirstPersonBP/Blueprints/FirstPersonCharacter` OtherActor)
  (`self.EnableInput` (`GameplayStatics.GetPlayerController` 0)))

(event `self.Box.OnComponentEndOverlap`
  (params (OverlappedComponent :type "PrimitiveComponent Object Reference") (OtherActor :type "Actor Object Reference") (OtherComp :type "PrimitiveComponent Object Reference") (OtherBodyIndex :type Integer))
  (cast `/Game/FirstPersonBP/Blueprints/FirstPersonCharacter` OtherActor)
  (`self.DisableInput` (`GameplayStatics.GetPlayerController` 0)))

(event `InputAction|use`
  (params (Key :type "Key Structure"))
  (:`Pressed`
    (if (== (`self.isOpen`) true)
      (`self.close`)
      (else
        (`self.open`)))))

(event `open`
  (bind (_direction _newtrack_0) (`Timeline|open_drawer` :!via `PlayFromStart`)
    (:`Update`
      (`SceneComponent.K2_SetRelativeLocation` (`self.drawer`) (`KismetMathLibrary.VLerp` (`SceneComponent.RelativeLocation` (`self.drawer`)) (-30.0 0.0 0.0) _newtrack_0) false false))
    (:`Finished`
      (set `self.isOpen` true))))

(event `close`
  (bind (_direction _newtrack_0) (`Timeline|Timeline_0` :!via `PlayFromStart`)
    (:`Update`
      (`SceneComponent.K2_SetRelativeLocation` (`self.drawer`) (`KismetMathLibrary.VLerp` (`SceneComponent.RelativeLocation` (`self.drawer`)) (0.0 0.0 0.0) _newtrack_0) false false))
    (:`Finished`
      (set `self.isOpen` false))))

(fn `UserConstructionScript`)