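; Trigger actor that toggles two groups of lights the first time a FirstPersonCharacter overlaps it.
; The overlap passes a cast and a DoOnce gate, then loops through LightsToOff toggling each light component's visibility.
; The LightsToOn loop is nested inside that loop, so its lights toggle and On_Cue plays at the Box location on every inner iteration.
; Visibility is flipped rather than set, so results depend on starting states and array sizes.
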(event `self.ReceiveActorBeginOverlap`
  (params (OtherActor :type "Actor Object Reference"))
  (cast `/Game/FirstPersonBP/Blueprints/FirstPersonCharacter` OtherActor)
  (`/Engine/EditorBlueprintResources/StandardMacros.DoOnce` false
    (:`Completed`
      (for _array_element (`self.LightsToOff`)
        (`SceneComponent.ToggleVisibility` (`Light.LightComponent` _array_element) false)
        (for _array_element_2 (`self.LightsToOn`)
          (`SceneComponent.ToggleVisibility` (`Light.LightComponent` _array_element_2) false)
          (`GameplayStatics.PlaySoundAtLocation` "/Game/Audio/Latarka/On_Cue.On_Cue" (`SceneComponent.K2_GetComponentLocation` (`self.Box`)) (struct) 1.0 1.0 0.0 null null null))))))

(fn `UserConstructionScript`)