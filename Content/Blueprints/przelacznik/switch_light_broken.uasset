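; Indicator light for a broken switch, which sets its PointLight to yellow or red from the state of a referenced SwitchActor.
; Two functions serve the cable (kable) and fuse (bezpiecznik) switch variants, each casting SwitchActor to its own class and reading IsBroken.
; A broken switch shows yellow and an unbroken one red.
; The event graph is inactive, so nothing in this Blueprint calls either function.
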(fn `SwitchLightRedOrYellowBezpiecznik`
  (bind _pointlight (`self.PointLight`))
  (bind _asbroken_switch_bezpiecznik (cast `/Game/Blueprints/PickUp/broken_switch_bezpiecznik` (`self.switch_actor`)))
  (if (`/Game/Blueprints/PickUp/broken_switch_bezpiecznik.is_broken` _asbroken_switch_bezpiecznik)
    (`LightComponent.SetLightColor` _pointlight (struct :`R` 255.0 :`G` 165.0 :`A` 1.0) true)
    (else
      (`LightComponent.SetLightColor` _pointlight (struct :`R` 255.0 :`A` 1.0) true))))

(fn `SwitchLightRedOrYellowKable`
  (bind _pointlight (`self.PointLight`))
  (bind _asbroken_switch_kable (cast `/Game/Blueprints/PickUp/broken_switch_kable` (`self.switch_actor`)))
  (if (`/Game/Blueprints/PickUp/broken_switch_kable.is_broken` _asbroken_switch_kable)
    (`LightComponent.SetLightColor` _pointlight (struct :`R` 255.0 :`G` 165.0 :`A` 1.0) true)
    (else
      (`LightComponent.SetLightColor` _pointlight (struct :`R` 255.0 :`A` 1.0) true))))

(fn `UserConstructionScript`
  (`parent.UserConstructionScript`))