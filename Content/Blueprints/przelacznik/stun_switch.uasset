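; Interactable stun switch that stuns nearby Mob_Ai enemies when the player uses it.
; Box overlap with FirstPersonCharacter shows a PressE widget and enables input.
; Use stuns mobs within range of any Stun_switch in the level; only such hits trigger all Stun_light actors and the handle timeline.
; The timeline's value moves the handle, switches lights off within a value window, and gates reuse through a Tick check.
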(event `self.Box.OnComponentBeginOverlap`
  (params (OverlappedComponent :type "PrimitiveComponent Object Reference") (OtherActor :type "Actor Object Reference") (OtherComp :type "PrimitiveComponent Object Reference") (OtherBodyIndex :type Integer) (bFromSweep :type Boolean) (SweepResult :type "HitResult Structure (by ref)"))
  (bind _returnvalue (`GameplayStatics.GetPlayerController` 0))
  (cast `/Game/FirstPersonBP/Blueprints/FirstPersonCharacter` OtherActor)
  (bind _returnvalue_2 (`|CreateWidget` "/Game/HUD/PressE.PressE_C" _returnvalue))
  (`UserWidget.AddToViewport` _returnvalue_2 0)
  (`self.EnableInput` _returnvalue))

(event `self.Box.OnComponentEndOverlap`
  (params (OverlappedComponent :type "PrimitiveComponent Object Reference") (OtherActor :type "Actor Object Reference") (OtherComp :type "PrimitiveComponent Object Reference") (OtherBodyIndex :type Integer))
  (cast `/Game/FirstPersonBP/Blueprints/FirstPersonCharacter` OtherActor)
  (`Widget.RemoveFromParent` (stale `self.Box.OnComponentBeginOverlap` _returnvalue_2))
  (`self.DisableInput` (`GameplayStatics.GetPlayerController` 0)))

(event `InputAction|use`
  (params (Key :type "Key Structure"))
  (bind (_relativelocation_x _relativelocation_y) (`KismetMathLibrary.BreakVector` (`SceneComponent.RelativeLocation` (`self.switch_handle`))))
  (:`Pressed`
    (if (`self.can_switch`)
      (set `self.is_on` true)
      (`GameplayStatics.PlaySoundAtLocation` "/Game/Audio/przelacznik/stun_switch.stun_switch" (`SceneComponent.RelativeLocation` (`self.base`)) (struct) 1.0 1.0 0.0 null null null)
      (bind _outactors (`GameplayStatics.GetAllActorsOfClass` "stun_switch_C"))
      (for _array_element _outactors
        (bind _outactors_2 (`GameplayStatics.GetAllActorsOfClass` "/Game/ThirdPersonBP/AI/Mob_Ai.Mob_Ai_C"))
        (for _array_element_2 _outactors_2
          (if (< (`KismetMathLibrary.Vector_Distance` (`self.K2_GetActorLocation` _array_element_2) (`self.K2_GetActorLocation` _array_element)) 7000.0)
            (`/Game/ThirdPersonBP/AI/Mob_Ai.stun` _array_element_2)
            (bind _outactors_3 (`GameplayStatics.GetAllActorsOfClass` "/Game/Blueprints/przelacznik/stun_light.stun_light_C"))
            (for _array_element_3 _outactors_3
              (`/Game/Blueprints/przelacznik/stun_light.StunLight` _array_element_3)
              (bind (_direction _switched) (`Timeline|Timeline_0` :!via `PlayFromStart`)
                (:`Update`
                  (`SceneComponent.K2_SetRelativeLocation` (`self.switch_handle`) (`KismetMathLibrary.MakeVector` _relativelocation_x _relativelocation_y _switched) false false)
                  (if (and (< _switched 20.0) (> _switched 16.0))
                    (for _array_element_4 _outactors_3
                      (`/Game/Blueprints/przelacznik/stun_light.StunLightOff` _array_element_4))))))))))))

(event `self.ReceiveTick`
  (params (DeltaSeconds :type "Float (single-precision)"))
  (set `self.can_switch` (not (and (< (stale `InputAction|use` _switched) 125.0) (> (stale `InputAction|use` _switched) 16.0)))))

(fn `UserConstructionScript`)