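; Stun light actor with a SpotLight whose visibility is tied to a referenced stun_switch actor.
; On BeginPlay it casts that actor and matches the spotlight's visibility to the switch's IsOn state, then hides the light after a short delay regardless of that state.
; StunLight and StunLightOff functions show and hide the spotlight directly.
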(event `self.ReceiveBeginPlay`
  (bind _spotlight (`self.SpotLight`))
  (bind _asstun_switch (cast `/Game/Blueprints/PickUp/stun_switch` (`self.stun_switch_actor`)))
  (`SceneComponent.SetVisibility` _spotlight (`/Game/Blueprints/PickUp/stun_switch.is_on` _asstun_switch) false)
  (`KismetSystemLibrary.Delay` 2.0)
  (`SceneComponent.SetVisibility` _spotlight false false))

(fn `StunLight`
  (`SceneComponent.SetVisibility` (`self.SpotLight`) true false))

(fn `StunLightOff`
  (`SceneComponent.SetVisibility` (`self.SpotLight`) false false))

(fn `UserConstructionScript`)