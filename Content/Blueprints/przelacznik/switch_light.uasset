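; Indicator light Blueprint that turns its PointLight green to reflect the state of a linked switch.
; SwitchLight casts the SwitchActor reference to switch_nowy and sets the green color when SwitchEnabled is true, with no branch for the disabled state.
; Nothing in this Blueprint calls SwitchLight: BeginPlay is empty, and the remaining color and visibility nodes are disconnected.
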(event `self.ReceiveBeginPlay`)

(fn `SwitchLight`
  (bind _asswitch_nowy (cast `/Game/Blueprints/PickUp/switch_nowy` (`self.switch_actor`)))
  (if (`/Game/Blueprints/PickUp/switch_nowy.switch_enabled` _asswitch_nowy)
    (`LightComponent.SetLightColor` (`self.PointLight`) (struct :`G` 255.0 :`A` 1.0) true)))

(fn `UserConstructionScript`)