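; Invisible door-item trigger variant that grants a door item and fires a one-time neighbour check event.
; When the first-person character overlaps its box, a DoOnce inserts true into the player's DoorItems array at DoorItemValue.
; It then spawns an EventLight at a hard-coded world position, briefly shows the NeighbourCheck widget after a delay, and destroys itself.
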(event `self.box.OnComponentBeginOverlap`
  (params (OverlappedComponent :type "PrimitiveComponent Object Reference") (OtherActor :type "Actor Object Reference") (OtherComp :type "PrimitiveComponent Object Reference") (OtherBodyIndex :type Integer) (bFromSweep :type Boolean) (SweepResult :type "HitResult Structure (by ref)"))
  (cast `/Game/FirstPersonBP/Blueprints/FirstPersonCharacter` OtherActor)
  (`/Engine/EditorBlueprintResources/StandardMacros.DoOnce` false
    (:`Completed`
      (bind _asfirst_person_character (cast `/Game/FirstPersonBP/Blueprints/FirstPersonCharacter` (`GameplayStatics.GetPlayerCharacter` 0)))
      (`KismetArrayLibrary.Array_Insert` (`/Game/FirstPersonBP/Blueprints/FirstPersonCharacter.door_items` _asfirst_person_character) true (`self.door_item_value`))
      (`|SpawnActorFromClass` "/Game/effects/EventLight.EventLight_C" (`KismetMathLibrary.Conv_VectorToTransform` (5953.0 82077.0 471.0)) "Undefined" "OverrideRootScale" null null)
      (`KismetSystemLibrary.Delay` 1.8)
      (bind _returnvalue (`|CreateWidget` "/Game/HUD/Subtitles/NeighbourCheck.NeighbourCheck_C"))
      (`UserWidget.AddToViewport` _returnvalue 0)
      (`KismetSystemLibrary.Delay` 3.0)
      (`Widget.RemoveFromParent` _returnvalue)
      (`self.K2_DestroyActor`))))

(fn `UserConstructionScript`
  (`parent.UserConstructionScript`))